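; BP_MetalEndRoom is a self-destroying actor that shows a moving rock undergoing a gold transmutation effect.
; On BeginPlay it randomizes the rock's rotation, creates a dynamic M_GoldTransmutation material and starts the Moving timeline.
; The timeline drives the rock's Y and Z location and the LerpMetal material parameter.
; Its Magic event track attaches the PS_GlowTrans glow effect to the rock, and the actor is destroyed when the timeline finishes.
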(event `self.ReceiveBeginPlay`
  (bind _rock (`self.Rock`))
  (`SceneComponent.K2_SetRelativeRotation` _rock (`KismetMathLibrary.RandomRotator` false) false false)
  (bind _returnvalue (`PrimitiveComponent.CreateDynamicMaterialInstance` _rock 0 "/Game/Materials/M_GoldTransmutation.M_GoldTransmutation" "None"))
  (set `self.MatRef` _returnvalue)
  (bind (_direction _moving _upanddown _trans) (`Timeline|Moving` :!via `PlayFromStart`)
    (:`Update`
      (`SceneComponent.K2_SetRelativeLocation` (`self.Rock`) (`KismetMathLibrary.MakeVector` 0.0 (* _moving -1.0) _upanddown) false false)
      (`MaterialInstanceDynamic.SetScalarParameterValue` (`self.MatRef`) "LerpMetal" _trans))
    (:`Finished`
      (`self.K2_DestroyActor`))
    (:`MagicEvent`
      (`NiagaraFunctionLibrary.SpawnSystemAttached` "/Game/Blueprints/Particles/PS_GlowTrans.PS_GlowTrans" (`self.Rock`) "None" (0.0 0.0 0.0) (struct) "KeepRelativeOffset"))))

(fn `UserConstructionScript`)