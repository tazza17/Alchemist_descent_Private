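; BP_LavaRising is a rising lava hazard whose climb to a target marker ends the level.
; LevelStart repeatedly sets a height just above the current one, which Tick lerps toward, then sends LevelCompleteMessage shortly after reaching the target.
; Overlap triggers the player's LavaTransition and flags the challenge failed, or deals lethal damage to enemies.
; The construction script sizes the lava's footprint from LavaX and LavaY.
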(event `self.ReceiveTick`
  (params (DeltaSeconds :type "Float (single-precision)"))
  (bind (_relativelocation_x _relativelocation_y _relativelocation_z) (`KismetMathLibrary.BreakVector` (`SceneComponent.RelativeLocation` (`self.LavaVol`))))
  (`SceneComponent.K2_SetRelativeLocation` (`self.LavaVol`) (`KismetMathLibrary.MakeVector` 0.0 0.0 (`KismetMathLibrary.Lerp` _relativelocation_z (`self.CurrentHeight`) 0.1)) false false))

(event `/Game/Blueprints/FrameWork/Interface_PP.LevelStart`
  (bind (_relativelocation_x _relativelocation_y _relativelocation_z) (`KismetMathLibrary.BreakVector` (`SceneComponent.RelativeLocation` (`self.LavaVol`))))
  (bind (_relativelocation_x_2 _relativelocation_y_2 _relativelocation_z_2) (`KismetMathLibrary.BreakVector` (`SceneComponent.RelativeLocation` (`self.RiseTargetPos`))))
  (set `self.CurrentHeight` (+ _relativelocation_z (`self.RiseSpeed`)) :!label _label)
  (`KismetSystemLibrary.Delay` 0.1)
  (if (>= _relativelocation_z _relativelocation_z_2)
    (`KismetSystemLibrary.Delay` 3.0)
    (message `/Game/Blueprints/FrameWork/Interface_PP.LevelComplete` (`GameplayStatics.GetGameInstance`))
    (else
      (goto _label))))

(event `self.LavaVol.OnComponentBeginOverlap`
  (params (OverlappedComponent :type "PrimitiveComponent Object Reference") (OtherActor :type "Actor Object Reference") (OtherComp :type "PrimitiveComponent Object Reference") (OtherBodyIndex :type Integer) (bFromSweep :type Boolean) (SweepResult :type "HitResult Structure (by ref)"))
  (bind _asbp_player_character (cast `/Game/Blueprints/Actors/BP_PlayerCharacter` OtherActor)
    (:`then`
      (`/Game/Blueprints/Actors/BP_PlayerCharacter.LavaTransition` _asbp_player_character false self)
      (bind _asgame_instance_pp (cast `/Game/Blueprints/FrameWork/GameInstance_PP` (`GameplayStatics.GetGameInstance`)))
      (set `/Game/Blueprints/FrameWork/GameInstance_PP.CurrentChallengeFailed?` true _asgame_instance_pp))
    (:`CastFailed`
      (bind _asbp_enemy (cast `/Game/Blueprints/Actors/Enemies/BP_Enemy` OtherActor))
      (`GameplayStatics.ApplyDamage` _asbp_enemy 999.0)
      (`KismetSystemLibrary.PrintString` "enemy died to lava"))))

(fn `CheckForSpaceHUD`
  (returns (`AnySpace?` :type Boolean) (EmptySlot :type "/Game/Blueprints/Widgets/WBP_HotbarSlot Object Reference"))
  (return false null))

(fn `ChooseRandomEnemy`
  (params (AlreadySelectedEnemy :type "/Game/Blueprints/Actors/Enemies/BP_Enemy Class Reference"))
  (returns (ChosenEnemy :type "/Game/Blueprints/Actors/Enemies/BP_Enemy Class Reference") (SpawnModifiers :type "/Game/Blueprints/FrameWork/S_EnemyModifiers Structure"))
  (return null))

(fn `GetChestItem`
  (params (Rarity :type Integer))
  (returns (ItemReceived :type "/Game/Blueprints/Actors/Interactables/Pickups/BP_PickUp Class Reference"))
  (return null))

(fn `GetPlayerStats`
  (returns (PlayerStats :type "/Game/Blueprints/FrameWork/S_PlayerStats Structure") (CurrentTime :type "Float (double-precision)"))
  (return (struct) 0.0))

(fn `GetRandomLevel`
  (params (LevelType :type "/Game/Blueprints/FrameWork/Enum_PortalTypes Enum" :default "NewEnumerator0"))
  (returns (ChosenLevel :type Name))
  (return "None"))

(fn `UserConstructionScript`
  (bind (_returnvalue_x _returnvalue_y _returnvalue_z) (`KismetMathLibrary.BreakVector` (`SceneComponent.K2_GetComponentLocation` (`self.RiseTargetPos`))))
  (`self.SetActorScale3D` (1.0 1.0 1.0))
  (set `self.RiseHeight` _returnvalue_z)
  (`SceneComponent.SetRelativeScale3D` (`self.LavaVol`) (`KismetMathLibrary.MakeVector` (`self.LavaX`) (`self.LavaY`) 1.0)))