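; BP_ChallengeTotem is an actor that shows the result of a challenge through the color of its cube.
; On LevelComplete it reads CurrentChallengeFailed from GameInstance_PP and swaps the cube material to red glass for failure or blue glass otherwise.
; The other functions, covering HUD space, enemy, chest item, player stats and level selection, are empty stubs, and the actor does no work on BeginPlay or Tick.
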(event `/Game/Blueprints/FrameWork/Interface_PP.LevelComplete`
  (bind _cube (`self.Cube`))
  (bind _asgame_instance_pp (cast `/Game/Blueprints/FrameWork/GameInstance_PP` (`GameplayStatics.GetGameInstance`)))
  (if (`/Game/Blueprints/FrameWork/GameInstance_PP.CurrentChallengeFailed?` _asgame_instance_pp)
    (`PrimitiveComponent.SetMaterial` _cube 0 "/Game/Materials/MI_Glass_Red.MI_Glass_Red")
    (else
      (`PrimitiveComponent.SetMaterial` _cube 0 "/Game/Materials/MI_Glass_Blue.MI_Glass_Blue"))))

(fn `CheckForSpaceHUD`
  (returns (`AnySpace?` :type Boolean) (EmptySlot :type "/Game/Blueprints/Widgets/WBP_HotbarSlot Object Reference"))
  (return false null))

(fn `ChooseRandomEnemy`
  (params (AlreadySelectedEnemy :type "/Game/Blueprints/Actors/Enemies/BP_Enemy Class Reference"))
  (returns (ChosenEnemy :type "/Game/Blueprints/Actors/Enemies/BP_Enemy Class Reference") (SpawnModifiers :type "/Game/Blueprints/FrameWork/S_EnemyModifiers Structure"))
  (return null))

(fn `GetChestItem`
  (params (Rarity :type Integer))
  (returns (ItemReceived :type "/Game/Blueprints/Actors/Interactables/Pickups/BP_PickUp Class Reference"))
  (return null))

(fn `GetPlayerStats`
  (returns (PlayerStats :type "/Game/Blueprints/FrameWork/S_PlayerStats Structure") (CurrentTime :type "Float (double-precision)"))
  (return (struct) 0.0))

(fn `GetRandomLevel`
  (params (LevelType :type "/Game/Blueprints/FrameWork/Enum_PortalTypes Enum" :default "NewEnumerator0"))
  (returns (ChosenLevel :type Name))
  (return "None"))

(fn `UserConstructionScript`)