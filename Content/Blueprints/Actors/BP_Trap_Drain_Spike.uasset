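; BP_Trap_Drain_Spike is a spike trap actor that reacts to the player's presence.
; Player_Indicator overlap with BP_PlayerCharacter plays the SpikeTrap timeline to move the spike along relative Z, and leaving reverses it.
; Each transition plays a 2D sound, slightly delayed on exit.
; A separate Spike_Damage overlap applies fixed damage to any actor entering it, independent of the trigger.
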(event `Shoot_Spike`
  (bind (_direction _newtrack_0) (`Timeline|Spike Trap` :!label _label)
    (:`Update`
      (`SceneComponent.K2_SetRelativeLocation` (`self.Spike`) (`KismetMathLibrary.MakeVector` 0.0 0.0 _newtrack_0) false false))))

(event `Close Spike`
  (goto _label :!via `Reverse`))

(event `self.Player_Indicator.OnComponentBeginOverlap`
  (params (OverlappedComponent :type "PrimitiveComponent Object Reference") (OtherActor :type "Actor Object Reference") (OtherComp :type "PrimitiveComponent Object Reference") (OtherBodyIndex :type Integer) (bFromSweep :type Boolean) (SweepResult :type "HitResult Structure (by ref)"))
  (cast `/Game/Blueprints/Actors/BP_PlayerCharacter` OtherActor)
  (`self.Shoot_Spike`)
  (`GameplayStatics.PlaySound2D` "/Game/Audio/Spike_Trap_Close_Sound_Effect.Spike_Trap_Close_Sound_Effect" 1.0 1.0 0.0 null null))

(event `self.Player_Indicator.OnComponentEndOverlap`
  (params (OverlappedComponent :type "PrimitiveComponent Object Reference") (OtherActor :type "Actor Object Reference") (OtherComp :type "PrimitiveComponent Object Reference") (OtherBodyIndex :type Integer))
  (cast `/Game/Blueprints/Actors/BP_PlayerCharacter` OtherActor)
  (`self.Close Spike`)
  (`KismetSystemLibrary.Delay` 0.2)
  (`GameplayStatics.PlaySound2D` "/Game/Audio/Spike_Trap_Open_Sound_Effect.Spike_Trap_Open_Sound_Effect" 1.0 1.0 0.0 null null))

(event `self.Spike_Damage.OnComponentBeginOverlap`
  (params (OverlappedComponent :type "PrimitiveComponent Object Reference") (OtherActor :type "Actor Object Reference") (OtherComp :type "PrimitiveComponent Object Reference") (OtherBodyIndex :type Integer) (bFromSweep :type Boolean) (SweepResult :type "HitResult Structure (by ref)"))
  (`GameplayStatics.ApplyDamage` OtherActor 15.0))

(fn `UserConstructionScript`)