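; BP_MagnumOpus is the game-ending interactable, a crystal that floats on a timeline from BeginPlay.
; On first interaction it stops the idle float and raises the crystal from its current height with a second timeline, while the HUD fades to white.
; When the rise finishes, it tells the Game Instance to show the game complete message.
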(event `self.ReceiveBeginPlay`
  (`parent.ReceiveBeginPlay`)
  (set `self.Used?` false)
  (bind (_direction _flaitoign) (`Timeline|Float` :!via `PlayFromStart` :!label _label)
    (:`Update`
      (`SceneComponent.K2_SetRelativeLocation` (`self.Crystal`) (`KismetMathLibrary.MakeVector` 0.0 0.0 _flaitoign) false false))))

(event `self.WhenInteractedWith`
  (bind _crystal (`self.Crystal`))
  (bind (_relativelocation_x _relativelocation_y _relativelocation_z) (`KismetMathLibrary.BreakVector` (`SceneComponent.RelativeLocation` _crystal)))
  (if (not (`self.Used?`))
    (set `self.Used?` true)
    (`|ExecutionSequence`
      (:`then_0`
        (goto _label :!via `Stop`))
      (:`then_1`
        (set `self.TempZ` _relativelocation_z)
        (bind (_direction _upwatds) (`Timeline|FloatingUpwards` :!via `PlayFromStart`)
          (:`Update`
            (`SceneComponent.K2_SetRelativeLocation` _crystal (`KismetMathLibrary.MakeVector` 0.0 0.0 (+ (`self.TempZ`) _upwatds)) false false))
          (:`Finished`
            (message `/Game/Blueprints/FrameWork/Interface_PP.GameComplete` (`GameplayStatics.GetGameInstance`)))))
      (:`then_2`
        (bind _ashud_pp (cast `/Game/Blueprints/FrameWork/HUD_PP` (`PlayerController.GetHUD` (`GameplayStatics.GetPlayerController` 0))))
        (`/Game/Blueprints/Widgets/WBP_HUD.FadeToWhiteEvent` (`/Game/Blueprints/FrameWork/HUD_PP.HUDREF` _ashud_pp))))))

(fn `UserConstructionScript`
  (`parent.UserConstructionScript`))