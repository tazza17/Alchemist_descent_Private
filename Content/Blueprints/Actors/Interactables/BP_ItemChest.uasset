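; Interactable treasure chest that, on first use, animates its lid open and reveals a random item pickup.
; Chained timelines rotate the lid, then float and scale the spawned item before marking the chest empty and clearing its overlay material.
; ChooseRandomRarity uses a weighted roll with a GameInstance pity counter guaranteeing the higher tier after repeated misses; the GameInstance maps rarity to item class.
; Opening sounds play on every interaction, even once opened.
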(event `self.WhenInteractedWith`
  (bind _returnvalue (`self.K2_GetActorLocation`))
  (bind _pickupitem (`self.PickupItem`))
  (bind _pickupitem_2 (`self.PickupItem`))
  (bind _returnvalue_location (`KismetMathLibrary.BreakTransform` (`SceneComponent.GetRelativeTransform` _pickupitem)))
  (`GameplayStatics.PlaySoundAtLocation` "/Game/Audio/Chest_EnchmentStarter.Chest_EnchmentStarter" _returnvalue (struct) 0.25 1.0 0.0 "/Game/Audio/PP_SoundAttenuation300.PP_SoundAttenuation300" null null null)
  (`GameplayStatics.PlaySoundAtLocation` "/Game/Audio/Chest_Enchmentloop.Chest_Enchmentloop" _returnvalue (struct) 0.25 1.0 0.0 "/Game/Audio/PP_SoundAttenuation300.PP_SoundAttenuation300" null null null)
  (if (not (`self.Opened?`))
    (set `self.Opened?` true)
    (bind (_direction _openangle) (`Timeline|LidOpening` :!via `PlayFromStart`)
      (:`Update`
        (`SceneComponent.K2_SetRelativeRotation` (`self.Lid`) (`KismetMathLibrary.MakeRotator` 180.0 _openangle 180.0) false false))
      (:`Finished`
        (bind _rarity (`self.ChooseRandomRarity` 0.0))
        (bind _itemreceived (message `/Game/Blueprints/FrameWork/Interface_PP.GetChestItem` (`GameplayStatics.GetGameInstance`) _rarity))
        (bind _returnvalue_2 (`|SpawnActorFromClass` _itemreceived (`KismetMathLibrary.MakeTransform` _returnvalue_location) "AlwaysSpawn" "MultiplyWithRoot" null null))
        (`self.K2_AttachToComponent` _returnvalue_2 _pickupitem "None" "KeepRelative" "KeepRelative" "KeepRelative" false)
        (bind (_direction_2 _size _floating) (`Timeline|RevealItem` :!via `PlayFromStart`)
          (:`Update`
            (`SceneComponent.K2_SetRelativeLocation` _pickupitem_2 (`KismetMathLibrary.MakeVector` 0.0 0.0 _floating) false false)
            (`SceneComponent.SetRelativeScale3D` _pickupitem_2 (`KismetMathLibrary.MakeVector` _size _size _size)))
          (:`Finished`
            (set `self.ObjectName` "Treasure Chest (empty)")
            (`MeshComponent.SetOverlayMaterial` (`self.Base`) null)
            (`MeshComponent.SetOverlayMaterial` (`self.Lid`) null)))))))

(fn `ChooseRandomRarity`
  (params (RarityBonus :type "Float (double-precision)"))
  (returns (Rarity :type Integer))
  (bind _asgame_instance_pp (cast `/Game/Blueprints/FrameWork/GameInstance_PP` (`GameplayStatics.GetGameInstance`)))
  (bind _chestluck (`/Game/Blueprints/FrameWork/GameInstance_PP.ChestLuck` _asgame_instance_pp))
  (if (>= _chestluck 4)
    (set `/Game/Blueprints/FrameWork/GameInstance_PP.ChestLuck` 0 _asgame_instance_pp)
    (return 2)
    (elif (<= (+ (`KismetMathLibrary.RandomFloatInRange` 0.0 100.0) RarityBonus) 70.0)
      (set `/Game/Blueprints/FrameWork/GameInstance_PP.ChestLuck` (+ _chestluck 1) _asgame_instance_pp)
      (return 1)
      (else
        (set `/Game/Blueprints/FrameWork/GameInstance_PP.ChestLuck` 0 _asgame_instance_pp)
        (return 2)))))

(fn `UserConstructionScript`)