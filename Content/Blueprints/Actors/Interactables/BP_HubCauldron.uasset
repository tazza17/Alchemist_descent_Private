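; Hub cauldron interactable that shows a controls tutorial, or a congratulations message once the game has been beaten.
; BeginPlay reads the PPSave1 save to pick green or purple materials, the glow particle asset and the billboard sprite.
; When the player enters the sphere, a timeline raises the bubble, then swaps it for the billboard; leaving reverses this.
; Interacting calls LevelCompleteMessage on the game instance.
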(event `self.ReceiveBeginPlay`
  (bind _cauldron (`self.Cauldron`))
  (bind _ps_cauldronglow (`self.PS_CauldronGlow`))
  (bind _bubble (`self.Bubble`))
  (`parent.ReceiveBeginPlay`)
  (bind _returnvalue (`GameplayStatics.LoadGameFromSlot` "PPSave1"))
  (bind _asbp_save_game (cast `/Game/Blueprints/FrameWork/BP_SaveGame` _returnvalue))
  (if (`/Game/Blueprints/FrameWork/BP_SaveGame.HaveBeatenGame` _asbp_save_game)
    (`PrimitiveComponent.SetMaterial` _cauldron 1 "/Game/Materials/M_CauldronMagicNewGreen.M_CauldronMagicNewGreen")
    (`PrimitiveComponent.SetMaterial` _bubble 0 "/Game/Materials/M_CauldronMagicNewGreen.M_CauldronMagicNewGreen")
    (`NiagaraComponent.SetAsset` _ps_cauldronglow "/Game/Blueprints/Particles/PS_CauldronGlowPostGame.PS_CauldronGlowPostGame" true)
    (set `self.Billboard Image` "/Game/Sprites/CongratsMessage.CongratsMessage")
    (else
      (`PrimitiveComponent.SetMaterial` _cauldron 1 "/Game/Materials/M_CauldronMagicNewPurple.M_CauldronMagicNewPurple")
      (`PrimitiveComponent.SetMaterial` _bubble 0 "/Game/Materials/M_CauldronMagicNewPurple.M_CauldronMagicNewPurple")
      (`NiagaraComponent.SetAsset` _ps_cauldronglow "/Game/Blueprints/Particles/PS_CauldronGlowPreGame.PS_CauldronGlowPreGame" true)
      (set `self.Billboard Image` "/Game/Sprites/TutorialControls.TutorialControls")))
  (`BillboardComponent.SetSprite` (`self.HowToBillboard`) (`self.Billboard Image`)))

(event `self.WhenInteractedWith`
  (message `/Game/Blueprints/FrameWork/Interface_PP.LevelComplete` (`GameplayStatics.GetGameInstance`)))

(event `self.ReceiveTick`
  (params (DeltaSeconds :type "Float (single-precision)"))
  (`parent.ReceiveTick` DeltaSeconds))

(event `self.Sphere.OnComponentBeginOverlap`
  (params (OverlappedComponent :type "PrimitiveComponent Object Reference") (OtherActor :type "Actor Object Reference") (OtherComp :type "PrimitiveComponent Object Reference") (OtherBodyIndex :type Integer) (bFromSweep :type Boolean) (SweepResult :type "HitResult Structure (by ref)"))
  (bind _bubble (`self.Bubble`))
  (bind _howtobillboard (`self.HowToBillboard`))
  (cast `/Game/Blueprints/Actors/BP_PlayerCharacter` OtherActor)
  (bind (_direction _rising) (`Timeline|Rise` :!label _label)
    (:`Update`
      (`SceneComponent.K2_SetRelativeLocation` (`self.Bubble`) (`KismetMathLibrary.MakeVector` 0.0 0.0 _rising) false false))
    (:`Finished`
      (if (== _rising 0.0)
        (`SceneComponent.SetVisibility` _howtobillboard false false)
        (`SceneComponent.SetVisibility` _bubble true false)
        (else
          (`SceneComponent.SetVisibility` _howtobillboard true false)
          (`SceneComponent.SetVisibility` _bubble false false))))))

(event `self.Sphere.OnComponentEndOverlap`
  (params (OverlappedComponent :type "PrimitiveComponent Object Reference") (OtherActor :type "Actor Object Reference") (OtherComp :type "PrimitiveComponent Object Reference") (OtherBodyIndex :type Integer))
  (cast `/Game/Blueprints/Actors/BP_PlayerCharacter` OtherActor)
  (`SceneComponent.SetVisibility` (`self.HowToBillboard`) false false)
  (`SceneComponent.SetVisibility` (`self.Bubble`) true false)
  (goto _label :!via `Reverse`))

(fn `UserConstructionScript`
  (`parent.UserConstructionScript`))