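; BP_HealingCampfire is a single-use interactable campfire that heals the player.
; On first interaction it sets a Used flag, switches off its pink fire and plus-health effects, updates the campfire's overlay material, and renames itself as used.
; It then casts the player pawn to BP_PlayerCharacter and calls HealPlayer with its HealingAmount.
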(event `self.WhenInteractedWith`
  (if (not (`self.Used?`))
    (set `self.Used?` true)
    (`ActorComponent.SetActive` (`self.PS_PinkFire`) false false)
    (`MeshComponent.SetOverlayMaterial` (`self.Campfire`) null)
    (`ActorComponent.SetActive` (`self.Plus_Health`) false false)
    (set `self.ObjectName` "Campfire (used)")
    (bind _asbp_player_character (cast `/Game/Blueprints/Actors/BP_PlayerCharacter` (`GameplayStatics.GetPlayerPawn` 0)))
    (`/Game/Blueprints/Actors/BP_PlayerCharacter.HealPlayer` _asbp_player_character (`self.HealingAmount`))))

(fn `UserConstructionScript`
  (`parent.UserConstructionScript`))