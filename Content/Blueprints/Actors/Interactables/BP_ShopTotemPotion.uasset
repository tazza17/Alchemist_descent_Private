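; BP_ShopTotemPotion is an interactable shop totem that sells a random item from its loot pool when the player can afford its cost.
; A sale deducts money, presses the button and lowers the spawned item on an attached scene point, detaching it and unlocking the totem when the drop ends.
; Timelines flash the eye's dynamic material green for a sale or red for insufficient money, while Tick turns the eye toward the player camera.
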(event `NotEnoughMoney`
  ; Not Enough Money
  (`MaterialInstanceDynamic.SetVectorParameterValue` (`self.MatRef`) "EyeColour" (struct :`R` 1.0 :`A` 1.0))
  (bind (_direction _fade) (`Timeline|FadeRed` :!via `PlayFromStart`)
    (:`Update`
      (`MaterialInstanceDynamic.SetVectorParameterValue` (`self.MatRef`) "EyeColour" (make `LinearColor` 1.0 _fade _fade)))))

(event `self.ReceiveBeginPlay`
  (bind _returnvalue (`PrimitiveComponent.CreateDynamicMaterialInstance` (`self.Eye`) 0 "/Game/Materials/M_ShopTotemEye.M_ShopTotemEye" "None"))
  (set `self.MatRef` _returnvalue))

(event `SellItem`
  (bind _droppeditemspawn (`self.DroppedItemSpawn`))
  (bind _droppeditemspawn_2 (`self.DroppedItemSpawn`))
  (bind _buttoncollider (`self.ButtonCollider`))
  (bind _shoplootpool (`self.ShopLootpool`))
  (bind (_relativelocation_x _relativelocation_y) (`KismetMathLibrary.BreakVector` (`SceneComponent.RelativeLocation` _droppeditemspawn_2)))
  (bind (_relativelocation_x_2 _relativelocation_y_2 _relativelocation_z) (`KismetMathLibrary.BreakVector` (`SceneComponent.RelativeLocation` _buttoncollider)))
  ; Buying item
  (set `self.InUse` true)
  (`|ExecutionSequence`
    (:`then_0`
      (`MaterialInstanceDynamic.SetVectorParameterValue` (`self.MatRef`) "EyeColour" (struct :`R` 0.002045 :`G` 1.0 :`A` 1.0))
      (bind (_direction _fade _press) (`Timeline|FadeGreen` :!via `PlayFromStart`)
        (:`Update`
          (`MaterialInstanceDynamic.SetVectorParameterValue` (`self.MatRef`) "EyeColour" (make `LinearColor` _fade 1.0 _fade))
          (`SceneComponent.K2_SetRelativeLocation` _buttoncollider (`KismetMathLibrary.MakeVector` _press _relativelocation_y_2 _relativelocation_z) false false))))
    (:`then_1`
      (bind _asbp_player_character (cast `/Game/Blueprints/Actors/BP_PlayerCharacter` (`GameplayStatics.GetPlayerPawn` 0)))
      (`/Game/Blueprints/Actors/BP_PlayerCharacter.MoneyChange` _asbp_player_character (* (`self.Cost`) -1.0)))
    (:`then_2`
      (`KismetArrayLibrary.Array_Shuffle` _shoplootpool)
      (bind _returnvalue (`|SpawnActorFromClass` (`|GetArrayItem` _shoplootpool) (`KismetMathLibrary.MakeTransform` (`SceneComponent.K2_GetComponentLocation` _droppeditemspawn)) "AlwaysSpawn" "MultiplyWithRoot" null null))
      (`self.K2_AttachToComponent` _returnvalue _droppeditemspawn "None" "SnapToTarget" "KeepRelative" "KeepRelative" true)
      (bind (_direction_2 _fall) (`Timeline|Drop` :!via `PlayFromStart`)
        (:`Update`
          (`SceneComponent.K2_SetRelativeLocation` _droppeditemspawn_2 (`KismetMathLibrary.MakeVector` _relativelocation_x _relativelocation_y _fall) false false))
        (:`Finished`
          (`self.K2_DetachFromActor` _returnvalue "KeepWorld" "KeepWorld" "KeepRelative")
          (set `self.InUse` false))))))

(event `self.ReceiveTick`
  (params (DeltaSeconds :type "Float (single-precision)"))
  (bind _eye (`self.Eye`))
  (`SceneComponent.K2_SetWorldRotation` _eye (`KismetMathLibrary.FindLookAtRotation` (`SceneComponent.K2_GetComponentLocation` _eye) (`SceneComponent.K2_GetComponentLocation` (`self.GetComponentByClass` (`GameplayStatics.GetPlayerPawn` 0) "/Script/Engine.CameraComponent"))) false false))

(event `self.WhenInteractedWith`
  ; When interacted with
  (if (not (`self.InUse`))
    (bind _asbp_player_character (cast `/Game/Blueprints/Actors/BP_PlayerCharacter` (`GameplayStatics.GetPlayerPawn` 0)))
    (if (>= (`/Game/Blueprints/Actors/BP_PlayerCharacter.CurrentMoney` _asbp_player_character) (`self.Cost`))
      (`self.SellItem`)
      (else
        (`self.NotEnoughMoney`)))))

(fn `UserConstructionScript`)