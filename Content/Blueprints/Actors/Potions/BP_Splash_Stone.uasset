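; BP_Splash_Stone is a stone potion splash effect actor that plays its impact feedback as soon as it spawns.
; On BeginPlay it starts an earth camera shake on the first player, plays a randomly pitched rock sound and spawns a rock-spread particle system at its location.
; A timeline then drives the uniform relative scale of its Scene component through a Size track.
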(event `self.ReceiveBeginPlay`
  (bind _returnvalue (`self.K2_GetActorLocation`))
  (`parent.ReceiveBeginPlay`)
  (`PlayerController.ClientStartCameraShake` :`self` (`GameplayStatics.GetPlayerController` 0) :`Shake` "/Game/Blueprints/FrameWork/BP_CameraShakeEarth.BP_CameraShakeEarth_C")
  (`GameplayStatics.PlaySoundAtLocation` "/Game/Audio/A_RockSound.A_RockSound" _returnvalue (struct) 1.0 (`KismetMathLibrary.RandomFloatInRange` 0.7 1.1) 0.0 null null null null)
  (`NiagaraFunctionLibrary.SpawnSystemAtLocation` "/Game/Blueprints/Particles/PS_RockSpread.PS_RockSpread" _returnvalue)
  (bind (_direction _size) (`Timeline|Timeline` :!via `PlayFromStart`)
    (:`Update`
      (`SceneComponent.SetRelativeScale3D` (`self.Scene`) (`KismetMathLibrary.MakeVector` _size _size _size)))))

(fn `UserConstructionScript`
  (`parent.UserConstructionScript`))