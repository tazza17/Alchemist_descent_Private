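; BP_Splash_Volatile is the explosive splash of a volatile potion, playing particles, randomized sound and a camera shake on spawn.
; Its ColliderRadius stays active for 0.3 seconds before collision is disabled, giving a brief blast window.
; Overlapping characters are launched away from the center with a minimum upward velocity.
; BP_PlayerCharacter also takes damage, using the IgnoreInvincibilityType damage type.
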(event `self.ReceiveBeginPlay`
  (bind _returnvalue (`self.K2_GetActorLocation`))
  (bind _returnvalue_2 (`KismetMathLibrary.RandomFloatInRange` 0.9 1.1))
  (`parent.ReceiveBeginPlay`)
  (`NiagaraFunctionLibrary.SpawnSystemAtLocation` "/Game/Blueprints/Particles/PS_ExplosionVolatile.PS_ExplosionVolatile" _returnvalue)
  (`GameplayStatics.PlaySoundAtLocation` "/Game/Audio/A_Explosion.A_Explosion" _returnvalue (struct) _returnvalue_2 _returnvalue_2 0.1 null null null null)
  (`PlayerController.ClientStartCameraShake` :`self` (`GameplayStatics.GetPlayerController` 0) :`Shake` "/Game/Blueprints/FrameWork/BP_CameraShakeExplosion.BP_CameraShakeExplosion_C")
  (`KismetSystemLibrary.Delay` 0.3)
  (`PrimitiveComponent.SetCollisionEnabled` (`self.ColliderRadius`) "NoCollision"))

(event `self.ColliderRadius.OnComponentBeginOverlap`
  (params (OverlappedComponent :type "PrimitiveComponent Object Reference") (OtherActor :type "Actor Object Reference") (OtherComp :type "PrimitiveComponent Object Reference") (OtherBodyIndex :type Integer) (bFromSweep :type Boolean) (SweepResult :type "HitResult Structure (by ref)"))
  (`|ExecutionSequence`
    (:`then_0`
      (bind _ascharacter (cast `Character` OtherActor))
      (bind (_returnvalue_x _returnvalue_y _returnvalue_z) (`KismetMathLibrary.BreakVector` (* (`KismetMathLibrary.GetDirectionUnitVector` (`self.K2_GetActorLocation`) (`self.K2_GetActorLocation` _ascharacter)) (1000.0 1000.0 1000.0))))
      (`Character.LaunchCharacter` _ascharacter (`KismetMathLibrary.MakeVector` _returnvalue_x _returnvalue_y (`KismetMathLibrary.FClamp` _returnvalue_z 300.0 999999.0)) false false))
    (:`then_1`
      (bind _asbp_player_character (cast `/Game/Blueprints/Actors/BP_PlayerCharacter` OtherActor))
      (`GameplayStatics.ApplyDamage` _asbp_player_character 20.0 null null "/Game/Blueprints/FrameWork/IgnoreInvincibilityType.IgnoreInvincibilityType_C"))))

(fn `UserConstructionScript`
  (`parent.UserConstructionScript`))