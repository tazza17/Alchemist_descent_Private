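; BP_SpikeCircle is a short-lived potion effect actor that damages enemies caught in its circle of spikes.
; On BeginPlay, a Scale timeline drives the uniform relative scale of eight colliders, and the actor destroys itself when it finishes.
; Any BP_Enemy that begins overlapping the actor receives a fixed amount of damage; other actors are ignored.
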(event `self.ReceiveActorBeginOverlap`
  (params (OtherActor :type "Actor Object Reference"))
  (bind _asbp_enemy (cast `/Game/Blueprints/Actors/Enemies/BP_Enemy` OtherActor))
  (`GameplayStatics.ApplyDamage` _asbp_enemy 12.0))

(event `self.ReceiveBeginPlay`
  (bind (_direction _newtrack_0) (`Timeline|Scale`)
    (:`Update`
      (`SceneComponent.SetRelativeScale3D` (`self.Collider1`) (`KismetMathLibrary.MakeVector` _newtrack_0 _newtrack_0 _newtrack_0))
      (`SceneComponent.SetRelativeScale3D` (`self.Collider2`) (`KismetMathLibrary.MakeVector` _newtrack_0 _newtrack_0 _newtrack_0))
      (`SceneComponent.SetRelativeScale3D` (`self.Collider3`) (`KismetMathLibrary.MakeVector` _newtrack_0 _newtrack_0 _newtrack_0))
      (`SceneComponent.SetRelativeScale3D` (`self.Collider4`) (`KismetMathLibrary.MakeVector` _newtrack_0 _newtrack_0 _newtrack_0))
      (`SceneComponent.SetRelativeScale3D` (`self.Collider5`) (`KismetMathLibrary.MakeVector` _newtrack_0 _newtrack_0 _newtrack_0))
      (`SceneComponent.SetRelativeScale3D` (`self.Collider6`) (`KismetMathLibrary.MakeVector` _newtrack_0 _newtrack_0 _newtrack_0))
      (`SceneComponent.SetRelativeScale3D` (`self.Collider7`) (`KismetMathLibrary.MakeVector` _newtrack_0 _newtrack_0 _newtrack_0))
      (`SceneComponent.SetRelativeScale3D` (`self.Collider8`) (`KismetMathLibrary.MakeVector` _newtrack_0 _newtrack_0 _newtrack_0)))
    (:`Finished`
      (`self.K2_DestroyActor`))))

(fn `UserConstructionScript`)