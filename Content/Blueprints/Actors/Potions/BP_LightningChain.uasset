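; Lightning bolt actor from the potions set that damages an enemy, with a camera shake and pitch-varied thunder sound on spawn.
; Its capsule damages the first BP_Enemy to overlap, using a damage type named for ignoring invincibility, then stops hitting.
; On BeginPlay it has a coin-flip chance to spawn a copy of itself at the same location after a short random delay, producing random-length chains of strikes.
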(event `self.ReceiveBeginPlay`
  (bind _returnvalue (`self.K2_GetActorLocation`))
  (`PlayerController.ClientStartCameraShake` :`self` (`GameplayStatics.GetPlayerController` 0) :`Shake` "/Game/Blueprints/FrameWork/BP_CameraShakeBolt.BP_CameraShakeBolt_C")
  (`GameplayStatics.PlaySoundAtLocation` "/Game/Audio/A_Lightning.A_Lightning" _returnvalue (struct) 0.7 (`KismetMathLibrary.RandomFloatInRange` 0.8 1.2) 0.1 null null null null)
  (if (`KismetMathLibrary.RandomBoolWithWeight` 0.5)
    (`KismetSystemLibrary.Delay` (`KismetMathLibrary.RandomFloatInRange` 0.1 0.4))
    (`|SpawnActorFromClass` "BP_LightningChain_C" (`KismetMathLibrary.MakeTransform` _returnvalue) "AlwaysSpawn" "MultiplyWithRoot" null null)))

(event `self.Capsule.OnComponentBeginOverlap`
  (params (OverlappedComponent :type "PrimitiveComponent Object Reference") (OtherActor :type "Actor Object Reference") (OtherComp :type "PrimitiveComponent Object Reference") (OtherBodyIndex :type Integer) (bFromSweep :type Boolean) (SweepResult :type "HitResult Structure (by ref)"))
  (if (not (`self.AlreadyHit?`))
    (bind _asbp_enemy (cast `/Game/Blueprints/Actors/Enemies/BP_Enemy` OtherActor))
    (`GameplayStatics.ApplyDamage` _asbp_enemy (`self.Damage`) null null "/Game/Blueprints/FrameWork/IgnoreInvincibilityType.IgnoreInvincibilityType_C")
    (set `self.AlreadyHit?` true)))

(fn `UserConstructionScript`)