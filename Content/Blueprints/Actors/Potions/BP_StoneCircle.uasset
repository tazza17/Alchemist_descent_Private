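; BP_StoneCircle is a short-lived potion effect actor that forms a damaging ring of stone.
; On BeginPlay it starts an earth camera shake, plays a rock sound at random pitch and runs a Scale timeline.
; The timeline uniformly drives the scale of eight colliders, then destroys the actor when finished.
; Any BP_Enemy that begins overlapping the actor takes a fixed amount of damage.
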(event `self.ReceiveBeginPlay`
  (`PlayerController.ClientStartCameraShake` :`self` (`GameplayStatics.GetPlayerController` 0) :`Shake` "/Game/Blueprints/FrameWork/BP_CameraShakeEarth.BP_CameraShakeEarth_C")
  (`GameplayStatics.PlaySound2D` "/Game/Audio/A_RockSound.A_RockSound" 1.0 (`KismetMathLibrary.RandomFloatInRange` 0.8 1.1) 0.0 null null)
  (bind (_direction _newtrack_0) (`Timeline|Scale`)
    (:`Update`
      (`SceneComponent.SetRelativeScale3D` (`self.Collider8`) (`KismetMathLibrary.MakeVector` _newtrack_0 _newtrack_0 _newtrack_0))
      (`SceneComponent.SetRelativeScale3D` (`self.Collider7`) (`KismetMathLibrary.MakeVector` _newtrack_0 _newtrack_0 _newtrack_0))
      (`SceneComponent.SetRelativeScale3D` (`self.Collider6`) (`KismetMathLibrary.MakeVector` _newtrack_0 _newtrack_0 _newtrack_0))
      (`SceneComponent.SetRelativeScale3D` (`self.Collider5`) (`KismetMathLibrary.MakeVector` _newtrack_0 _newtrack_0 _newtrack_0))
      (`SceneComponent.SetRelativeScale3D` (`self.Collider4`) (`KismetMathLibrary.MakeVector` _newtrack_0 _newtrack_0 _newtrack_0))
      (`SceneComponent.SetRelativeScale3D` (`self.Collider2`) (`KismetMathLibrary.MakeVector` _newtrack_0 _newtrack_0 _newtrack_0))
      (`SceneComponent.SetRelativeScale3D` (`self.Collider3`) (`KismetMathLibrary.MakeVector` _newtrack_0 _newtrack_0 _newtrack_0))
      (`SceneComponent.SetRelativeScale3D` (`self.Collider1`) (`KismetMathLibrary.MakeVector` _newtrack_0 _newtrack_0 _newtrack_0)))
    (:`Finished`
      (`self.K2_DestroyActor`))))

(event `self.ReceiveActorBeginOverlap`
  (params (OtherActor :type "Actor Object Reference"))
  (bind _asbp_enemy (cast `/Game/Blueprints/Actors/Enemies/BP_Enemy` OtherActor))
  (`GameplayStatics.ApplyDamage` _asbp_enemy 7.0))

(fn `UserConstructionScript`)