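; BP_Splash_Healing is the healing potion splash actor, restoring health to characters that touch its radius.
; On BeginPlay it spawns the health splash particle system at its location.
; Overlapping the ColliderRadius component heals a player character through HealPlayer, and sends negative damage to an enemy through ApplyDamage, apparently to heal it by a smaller amount.
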(event `self.ReceiveBeginPlay`
  (`parent.ReceiveBeginPlay`)
  (`NiagaraFunctionLibrary.SpawnSystemAtLocation` "/Game/Blueprints/Particles/PS_HealthSplash.PS_HealthSplash" (`self.K2_GetActorLocation`)))

(event `self.ColliderRadius.OnComponentBeginOverlap`
  (params (OverlappedComponent :type "PrimitiveComponent Object Reference") (OtherActor :type "Actor Object Reference") (OtherComp :type "PrimitiveComponent Object Reference") (OtherBodyIndex :type Integer) (bFromSweep :type Boolean) (SweepResult :type "HitResult Structure (by ref)"))
  (`|ExecutionSequence`
    (:`then_0`
      (bind _asbp_player_character (cast `/Game/Blueprints/Actors/BP_PlayerCharacter` OtherActor))
      (`/Game/Blueprints/Actors/BP_PlayerCharacter.HealPlayer` _asbp_player_character 25.0))
    (:`then_1`
      (bind _asbp_enemy (cast `/Game/Blueprints/Actors/Enemies/BP_Enemy` OtherActor))
      (`GameplayStatics.ApplyDamage` _asbp_enemy -5.0))))

(fn `UserConstructionScript`
  (`parent.UserConstructionScript`))