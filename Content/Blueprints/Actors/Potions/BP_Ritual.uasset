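; BP_Ritual is a potion-spawned ritual actor that marks enemies for death when its animation completes.
; On BeginPlay a timeline spins the floor spell plane by yaw and scales the whole actor.
; When it finishes, it spawns a pentagram finish effect, calls MarkedForDeath on every BP_Enemy overlapping its collider, then destroys itself.
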(event `self.ReceiveBeginPlay`
  (bind _floorplanespell (`self.FloorPlaneSpell`))
  (bind (_relativerotation_roll _relativerotation_pitch _relativerotation_yaw) (`KismetMathLibrary.BreakRotator` (`SceneComponent.RelativeRotation` _floorplanespell)))
  (bind (_direction _spin _scale) (`Timeline|Animation`)
    (:`Update`
      (`SceneComponent.K2_SetRelativeRotation` _floorplanespell (`KismetMathLibrary.MakeRotator` 0.0 0.0 (+ _relativerotation_yaw _spin)) false false)
      (`self.SetActorScale3D` (`KismetMathLibrary.Conv_DoubleToVector` _scale)))
    (:`Finished`
      (`NiagaraFunctionLibrary.SpawnSystemAtLocation` "/Game/Blueprints/Particles/PS_PentagramFinish.PS_PentagramFinish" (`self.K2_GetActorLocation`))
      (for _array_element (`PrimitiveComponent.GetOverlappingActors` (`self.Collider`) "/Game/Blueprints/Actors/Enemies/BP_Enemy.BP_Enemy_C")
        (bind _asbp_enemy (cast `/Game/Blueprints/Actors/Enemies/BP_Enemy` _array_element))
        (`/Game/Blueprints/Actors/Enemies/BP_Enemy.MarkedForDeath` _asbp_enemy))
      (`self.K2_DestroyActor`))))

(fn `UserConstructionScript`)