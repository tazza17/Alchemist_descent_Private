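; BP_Splash_Storm is the splash effect actor of a storm potion, an air blast that knocks characters away.
; On BeginPlay it plays a pitch-randomized airburst sound and spawns an air blast particle system at its location.
; Characters that begin overlapping its ColliderRadius component are launched away from the actor's center, with vertical velocity clamped to a minimum so they always get some upward lift.
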(event `self.ReceiveBeginPlay`
  (bind _returnvalue (`self.K2_GetActorLocation`))
  (`parent.ReceiveBeginPlay`)
  (`GameplayStatics.PlaySoundAtLocation` "/Game/Audio/A_Airburst.A_Airburst" _returnvalue (struct) 1.0 (`KismetMathLibrary.RandomFloatInRange` 0.7 1.4) 0.09 null null null null)
  (`NiagaraFunctionLibrary.SpawnSystemAtLocation` "/Game/Blueprints/Particles/PS_AirBlastStrong.PS_AirBlastStrong" _returnvalue))

(event `self.ColliderRadius.OnComponentBeginOverlap`
  (params (OverlappedComponent :type "PrimitiveComponent Object Reference") (OtherActor :type "Actor Object Reference") (OtherComp :type "PrimitiveComponent Object Reference") (OtherBodyIndex :type Integer) (bFromSweep :type Boolean) (SweepResult :type "HitResult Structure (by ref)"))
  (bind _ascharacter (cast `Character` OtherActor))
  (bind (_returnvalue_x _returnvalue_y _returnvalue_z) (`KismetMathLibrary.BreakVector` (* (`KismetMathLibrary.GetDirectionUnitVector` (`self.K2_GetActorLocation`) (`self.K2_GetActorLocation` _ascharacter)) (800.0 800.0 800.0))))
  (`Character.LaunchCharacter` _ascharacter (`KismetMathLibrary.MakeVector` _returnvalue_x _returnvalue_y (`KismetMathLibrary.FClamp` _returnvalue_z 300.0 999999.0)) false false))

(fn `UserConstructionScript`
  (`parent.UserConstructionScript`))