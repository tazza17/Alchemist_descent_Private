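; BP_Splash is the impact actor for a thrown potion, producing the shatter and splash and affecting nearby enemies.
; On BeginPlay it plays a random-pitched glass shatter sound unless muted, then spawns shatter and splash particle systems, tinting the splash with its SplashColor.
; When a BP_Enemy begins overlapping its ColliderRadius, it deals BaseDamage and applies its PotionEffect to that enemy.
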(event `self.ReceiveBeginPlay`
  (bind _returnvalue (`self.K2_GetActorLocation`))
  (if (not (`self.MuteGlassSound`))
    (`GameplayStatics.PlaySoundAtLocation` "/Game/Audio/A_GlassShatter.A_GlassShatter" (`self.K2_GetActorLocation`) (struct) 1.0 (`KismetMathLibrary.RandomFloatInRange` 0.4 1.0) 0.1 null null null null))
  (`NiagaraFunctionLibrary.SpawnSystemAtLocation` "/Game/Blueprints/Particles/PS_GlassShatter.PS_GlassShatter" _returnvalue)
  (bind _returnvalue_2 (`NiagaraFunctionLibrary.SpawnSystemAtLocation` "/Game/Blueprints/Particles/PS_Splash.PS_Splash" _returnvalue))
  (`NiagaraComponent.SetVariableLinearColor` _returnvalue_2 "SplashColor" (`self.SplashColor`)))

(event `self.ColliderRadius.OnComponentBeginOverlap`
  (params (OverlappedComponent :type "PrimitiveComponent Object Reference") (OtherActor :type "Actor Object Reference") (OtherComp :type "PrimitiveComponent Object Reference") (OtherBodyIndex :type Integer) (bFromSweep :type Boolean) (SweepResult :type "HitResult Structure (by ref)"))
  (bind _asbp_enemy (cast `/Game/Blueprints/Actors/Enemies/BP_Enemy` OtherActor))
  (`GameplayStatics.ApplyDamage` _asbp_enemy (`self.BaseDamage`))
  (`/Game/Blueprints/Actors/Enemies/BP_Enemy.ApplyEffectsToEnemy` _asbp_enemy (`self.PotionEffect`)))

(fn `UserConstructionScript`)