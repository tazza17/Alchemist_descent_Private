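; BP_Kamikaze is a potion actor that charges up, then explodes, hurting the player to damage and knock back nearby enemies.
; On BeginPlay a Chargeup timeline grows the glowing sphere alongside a HUD animation.
; When it finishes, the player loses just under half max health, and an Explosion timeline expands the collision before destroying the actor.
; Overlapped enemies take invincibility-ignoring damage, receive an effect and are launched away with clamped, always-upward velocity.
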(event `self.ReceiveBeginPlay`
  (bind _returnvalue (`KismetMathLibrary.RandomFloatInRange` 0.9 1.1))
  (`PrimitiveComponent.SetCollisionEnabled` (`self.ExplosionCollision`) "NoCollision")
  (`GameplayStatics.PlaySound2D` "/Game/Audio/A_MagicChargeup.A_MagicChargeup" 1.0 1.0 0.0 null null)
  (bind _ashud_pp (cast `/Game/Blueprints/FrameWork/HUD_PP` (`PlayerController.GetHUD` (`GameplayStatics.GetPlayerController` 0))))
  (`/Game/Blueprints/Widgets/WBP_HUD.KamikazeAnim` (`/Game/Blueprints/FrameWork/HUD_PP.HUDREF` _ashud_pp))
  (bind (_direction _grow _brightness) (`Timeline|Chargeup` :!via `PlayFromStart`)
    (:`Update`
      (`SceneComponent.SetRelativeScale3D` (`self.Sphere`) (`KismetMathLibrary.MakeVector` _grow _grow _grow))
      (`LightComponent.SetIntensity` (`self.PointLight`) _brightness))
    (:`Finished`
      (`SceneComponent.SetVisibility` (`self.Sphere`) false false)
      (`ActorComponent.SetActive` (`self.Niagara`) false false)
      (bind _asbp_player_character (cast `/Game/Blueprints/Actors/BP_PlayerCharacter` (`GameplayStatics.GetPlayerPawn` 0)))
      (`GameplayStatics.ApplyDamage` _asbp_player_character (- (/ (`/Game/Blueprints/Actors/BP_PlayerCharacter.MaxHealth` _asbp_player_character) 2.0) 5.0) null null "/Game/Blueprints/FrameWork/IgnoreInvincibilityType.IgnoreInvincibilityType_C")
      (`NiagaraFunctionLibrary.SpawnSystemAtLocation` "/Game/Blueprints/Particles/PS_ExplosionKamikaze.PS_ExplosionKamikaze" (`self.K2_GetActorLocation`))
      (`PrimitiveComponent.SetCollisionEnabled` (`self.ExplosionCollision`) "QueryAndPhysics")
      (`PlayerController.ClientStartCameraShake` :`self` (`GameplayStatics.GetPlayerController` 0) :`Shake` "/Game/Blueprints/FrameWork/BP_CameraShakeKamikaze.BP_CameraShakeKamikaze_C")
      (`GameplayStatics.PlaySound2D` "/Game/Audio/A_Explosion.A_Explosion" _returnvalue _returnvalue 0.1 null null)
      (bind (_direction_2 _growcollision) (`Timeline|Explosion` :!via `PlayFromStart`)
        (:`Update`
          (`SceneComponent.SetWorldScale3D` (`self.ExplosionCollision`) (`KismetMathLibrary.MakeVector` _growcollision _growcollision _growcollision)))
        (:`Finished`
          (`self.K2_DestroyActor`))))))

(event `self.ExplosionCollision.OnComponentBeginOverlap`
  (params (OverlappedComponent :type "PrimitiveComponent Object Reference") (OtherActor :type "Actor Object Reference") (OtherComp :type "PrimitiveComponent Object Reference") (OtherBodyIndex :type Integer) (bFromSweep :type Boolean) (SweepResult :type "HitResult Structure (by ref)"))
  (bind _asbp_enemy (cast `/Game/Blueprints/Actors/Enemies/BP_Enemy` OtherActor))
  (`GameplayStatics.ApplyDamage` _asbp_enemy 50.0 null null "/Game/Blueprints/FrameWork/IgnoreInvincibilityType.IgnoreInvincibilityType_C")
  (message `/Game/Blueprints/FrameWork/Interface_PP.ApplyEffectsToEnemy` _asbp_enemy "NewEnumerator0")
  (bind (_returnvalue_x _returnvalue_y _returnvalue_z) (`KismetMathLibrary.BreakVector` (* (`KismetMathLibrary.GetDirectionUnitVector` (`self.K2_GetActorLocation`) (`self.K2_GetActorLocation` _asbp_enemy)) (500.0 500.0 500.0))))
  (`Character.LaunchCharacter` _asbp_enemy (`KismetMathLibrary.MakeVector` (`KismetMathLibrary.FClamp` _returnvalue_x -300.0 300.0) (`KismetMathLibrary.FClamp` _returnvalue_y -300.0 300.0) (`KismetMathLibrary.FClamp` _returnvalue_z 300.0 500.0)) false false))

(fn `UserConstructionScript`)