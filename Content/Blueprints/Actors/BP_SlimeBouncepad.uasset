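; A slime bounce pad actor that springs the player character upward.
; When BounceCollider is overlapped by BP_PlayerCharacter while it is falling, it launches the character straight up, overriding vertical velocity but keeping horizontal motion.
; The construction script sets the Slime mesh material from the GoopColour choice of green, red or blue, which affects only the look, not the bounce.
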(event `self.BounceCollider.OnComponentBeginOverlap`
  (params (OverlappedComponent :type "PrimitiveComponent Object Reference") (OtherActor :type "Actor Object Reference") (OtherComp :type "PrimitiveComponent Object Reference") (OtherBodyIndex :type Integer) (bFromSweep :type Boolean) (SweepResult :type "HitResult Structure (by ref)"))
  (bind _asbp_player_character (cast `/Game/Blueprints/Actors/BP_PlayerCharacter` OtherActor))
  (if (`NavMovementComponent.IsFalling` (`Character.CharacterMovement` _asbp_player_character))
    (`Character.LaunchCharacter` _asbp_player_character (0.0 0.0 900.0) false true)))

(fn `UserConstructionScript`
  (bind _slime (`self.Slime`))
  (switch `/Game/Blueprints/FrameWork/Enum_GoopColour` (`self.GoopColour`)
    (:`NewEnumerator0`
      (`PrimitiveComponent.SetMaterial` _slime 0 "/Game/Materials/M_Slime_Goop_Green.M_Slime_Goop_Green"))
    (:`NewEnumerator1`
      (`PrimitiveComponent.SetMaterial` _slime 0 "/Game/Materials/M_Slime_Goop_Red.M_Slime_Goop_Red"))
    (:`NewEnumerator2`
      (`PrimitiveComponent.SetMaterial` _slime 0 "/Game/Materials/M_Slime_Goop_Blue.M_Slime_Goop_Blue"))))