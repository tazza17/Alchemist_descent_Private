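; BP_BossFireball is a boss fireball projectile that explodes when its movement stops.
; The construction script independently randomizes its initial and max speed within a shared range.
; From BeginPlay, a looping short delay repeatedly spawns a fire particle system at its current location, forming a trail.
; On projectile stop, it spawns BP_BossExplosion at the impact point, passes on its Damage, then destroys itself a tick later.
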(event `self.ReceiveBeginPlay`
  (`NiagaraFunctionLibrary.SpawnSystemAtLocation` "/Game/Blueprints/Particles/PS_FireProjectile.PS_FireProjectile" (`self.K2_GetActorLocation`) :!label _label)
  (`KismetSystemLibrary.Delay` 0.05)
  (goto _label))

(event `self.ProjectileMovement.OnProjectileStop`
  (params (ImpactResult :type "HitResult Structure (by ref)"))
  (bind _returnvalue (`|SpawnActorFromClass` "/Game/Blueprints/Actors/Enemies/EnemyMisc/BP_BossExplosion.BP_BossExplosion_C" (`KismetMathLibrary.MakeTransform` ImpactResult_Location) "Undefined" "MultiplyWithRoot" null null))
  (set `/Game/Blueprints/Actors/Enemies/EnemyMisc/BP_BossExplosion.ExplosionDamage` (`self.Damage`) _returnvalue)
  (`KismetSystemLibrary.DelayUntilNextTick`)
  (`self.K2_DestroyActor`))

(fn `UserConstructionScript`
  (bind _returnvalue (`KismetMathLibrary.RandomFloatInRange` 800.0 1500.0))
  (bind _projectilemovement (`self.ProjectileMovement`))
  (set `ProjectileMovementComponent.InitialSpeed` _returnvalue _projectilemovement)
  (set `ProjectileMovementComponent.MaxSpeed` _returnvalue _projectilemovement))