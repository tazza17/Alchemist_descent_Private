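; Enemy spawn point actor that spawns a randomly chosen enemy when it receives LevelStart.
; It passes its Enemy class to the Game Instance, which returns the chosen enemy and spawn modifiers.
; SpawnEnemy always spawns at SpawnpointVector's location, then scales health, max health and attack damage by those modifiers and prints the health.
; The other functions are empty or return default values.
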(event `/Game/Blueprints/FrameWork/Interface_PP.LevelStart`
  (bind (_chosenenemy _spawnmodifiers) (message `/Game/Blueprints/FrameWork/Interface_PP.ChooseRandomEnemy` (`GameplayStatics.GetGameInstance`) (`self.Enemy`)))
  (set `self.Enemy` _chosenenemy)
  (set `self.SpawnedModifiers` _spawnmodifiers)
  (`self.SpawnEnemy`))

(event `SpawnEnemy`
  (bind (_spawnedmodifiers_hpmodifier _spawnedmodifiers_attackmodifier) (break `/Game/Blueprints/FrameWork/S_EnemyModifiers` (`self.SpawnedModifiers`)))
  (bind _returnvalue (`|SpawnActorFromClass` (`self.Enemy`) (`KismetMathLibrary.MakeTransform` (`SceneComponent.K2_GetComponentLocation` (`self.SpawnpointVector`))) "AlwaysSpawn" "MultiplyWithRoot" null null))
  (bind _output_get (set `self.SpawnedEnemy` _returnvalue))
  (bind _returnvalue_2 (* (`/Game/Blueprints/Actors/Enemies/BP_Enemy.EnemyMaxHealth` _output_get) _spawnedmodifiers_hpmodifier))
  (bind _output_get_2 (set `/Game/Blueprints/Actors/Enemies/BP_Enemy.EnemyHealth` _returnvalue_2 _output_get))
  (set `/Game/Blueprints/Actors/Enemies/BP_Enemy.EnemyMaxHealth` _returnvalue_2 _output_get)
  (set `/Game/Blueprints/Actors/Enemies/BP_Enemy.AttackDamage` (* (`/Game/Blueprints/Actors/Enemies/BP_Enemy.AttackDamage` _output_get) _spawnedmodifiers_attackmodifier) _output_get)
  (`KismetSystemLibrary.PrintString` (`KismetStringLibrary.Conv_DoubleToString` _output_get_2)))

(fn `CheckForSpaceHUD`
  (returns (`AnySpace?` :type Boolean) (EmptySlot :type "/Game/Blueprints/Widgets/WBP_HotbarSlot Object Reference"))
  (return false null))

(fn `ChooseRandomEnemy`
  (params (AlreadySelectedEnemy :type "/Game/Blueprints/Actors/Enemies/BP_Enemy Class Reference"))
  (returns (ChosenEnemy :type "/Game/Blueprints/Actors/Enemies/BP_Enemy Class Reference") (SpawnModifiers :type "/Game/Blueprints/FrameWork/S_EnemyModifiers Structure"))
  (return null))

(fn `GetChestItem`
  (params (Rarity :type Integer))
  (returns (ItemReceived :type "/Game/Blueprints/Actors/Interactables/Pickups/BP_PickUp Class Reference"))
  (return null))

(fn `GetPlayerStats`
  (returns (PlayerStats :type "/Game/Blueprints/FrameWork/S_PlayerStats Structure") (CurrentTime :type "Float (double-precision)"))
  (return (struct) 0.0))

(fn `GetRandomLevel`
  (params (LevelType :type "/Game/Blueprints/FrameWork/Enum_PortalTypes Enum" :default "NewEnumerator0"))
  (returns (ChosenLevel :type Name))
  (return "None"))

(fn `UserConstructionScript`)