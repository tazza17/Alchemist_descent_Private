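; BP_BossLightning is a telegraphed lightning strike hazard that damages the player.
; On spawn its capsule collision is off while a timeline grows a spinning plane as a warning marker.
; When the growth finishes it enables collision, spawns a bolt effect with camera shake and randomly pitched thunder, then destroys itself on the next tick.
; Player characters overlapping the capsule in that brief window take LightningDamage.
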(event `self.Capsule.OnComponentBeginOverlap`
  (params (OverlappedComponent :type "PrimitiveComponent Object Reference") (OtherActor :type "Actor Object Reference") (OtherComp :type "PrimitiveComponent Object Reference") (OtherBodyIndex :type Integer) (bFromSweep :type Boolean) (SweepResult :type "HitResult Structure (by ref)"))
  (bind _asbp_player_character (cast `/Game/Blueprints/Actors/BP_PlayerCharacter` OtherActor))
  (`GameplayStatics.ApplyDamage` _asbp_player_character (`self.LightningDamage`)))

(event `self.ReceiveTick`
  (params (DeltaSeconds :type "Float (single-precision)"))
  (`SceneComponent.K2_AddLocalRotation` (`self.Plane`) (struct :`Yaw` 5.0) false false))

(event `self.ReceiveBeginPlay`
  (bind _returnvalue (`self.K2_GetActorLocation`))
  (`PrimitiveComponent.SetCollisionEnabled` (`self.Capsule`) "NoCollision")
  (bind (_direction _growing) (`Timeline|Grow` :!via `PlayFromStart`)
    (:`Update`
      (`SceneComponent.SetRelativeScale3D` (`self.Plane`) (`KismetMathLibrary.MakeVector` _growing _growing _growing)))
    (:`Finished`
      (`PrimitiveComponent.SetCollisionEnabled` (`self.Capsule`) "QueryAndPhysics")
      (`NiagaraFunctionLibrary.SpawnSystemAtLocation` "/Game/Blueprints/Particles/PS_LightningBolt.PS_LightningBolt" _returnvalue)
      (`PlayerController.ClientStartCameraShake` :`self` (`GameplayStatics.GetPlayerController` 0) :`Shake` "/Game/Blueprints/FrameWork/BP_CameraShakeBolt.BP_CameraShakeBolt_C")
      (`GameplayStatics.PlaySoundAtLocation` "/Game/Audio/A_Lightning.A_Lightning" _returnvalue (struct) 0.5 (`KismetMathLibrary.RandomFloatInRange` 1.0 1.3) 0.0 null null null null)
      (`KismetSystemLibrary.DelayUntilNextTick`)
      (`self.K2_DestroyActor`))))

(fn `UserConstructionScript`)