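; BP_BossExplosion is an explosion actor, apparently for boss enemies, that damages the player on contact.
; On BeginPlay it spawns a volatile explosion effect, plays a quiet, low-pitched randomized sound and starts an earth camera shake on the first player.
; Tick polls the Collider for the player pawn and, after a one-tick delay, applies ExplosionDamage repeatedly while the overlap lasts.
; The graph contains no one-hit guard or destroy logic.
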(event `self.ReceiveBeginPlay`
  (bind _returnvalue (`self.K2_GetActorLocation`))
  (bind _returnvalue_2 (`KismetMathLibrary.RandomFloatInRange` 0.3 0.5))
  (`NiagaraFunctionLibrary.SpawnSystemAtLocation` "/Game/Blueprints/Particles/PS_ExplosionVolatile.PS_ExplosionVolatile" _returnvalue)
  (`GameplayStatics.PlaySoundAtLocation` "/Game/Audio/A_Explosion.A_Explosion" _returnvalue (struct) _returnvalue_2 _returnvalue_2 0.1 null null null null)
  (`PlayerController.ClientStartCameraShake` :`self` (`GameplayStatics.GetPlayerController` 0) :`Shake` "/Game/Blueprints/FrameWork/BP_CameraShakeEarth.BP_CameraShakeEarth_C"))

(event `self.ReceiveTick`
  (params (DeltaSeconds :type "Float (single-precision)"))
  (bind _returnvalue (`GameplayStatics.GetPlayerPawn` 0))
  (if (`PrimitiveComponent.IsOverlappingActor` (`self.Collider`) _returnvalue)
    (bind _asbp_player_character (cast `/Game/Blueprints/Actors/BP_PlayerCharacter` _returnvalue))
    (`KismetSystemLibrary.DelayUntilNextTick`)
    (`GameplayStatics.ApplyDamage` _asbp_player_character (`self.ExplosionDamage`))))

(fn `UserConstructionScript`)