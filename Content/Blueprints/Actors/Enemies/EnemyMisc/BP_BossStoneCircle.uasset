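; BP_BossStoneCircle is a short-lived boss attack hazard that damages the player on overlap.
; On BeginPlay it shakes the first player's camera and plays a rock sound with randomized volume and pitch.
; A Scale timeline drives the uniform scale of eight colliders together, then destroys the actor when it finishes.
; Overlaps with BP_PlayerCharacter apply the Damage value; other actors are ignored.
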(event `self.ReceiveBeginPlay`
  (bind _returnvalue (`KismetMathLibrary.RandomFloatInRange` 0.8 1.1))
  (`PlayerController.ClientStartCameraShake` :`self` (`GameplayStatics.GetPlayerController` 0) :`Shake` "/Game/Blueprints/FrameWork/BP_CameraShakeEarth.BP_CameraShakeEarth_C")
  (`GameplayStatics.PlaySoundAtLocation` "/Game/Audio/A_RockSound.A_RockSound" (0.0 0.0 0.0) (struct) _returnvalue _returnvalue 0.0 null null null null)
  (bind (_direction _newtrack_0) (`Timeline|Scale` :!via `PlayFromStart`)
    (:`Update`
      (`SceneComponent.SetRelativeScale3D` (`self.Collider8`) (`KismetMathLibrary.MakeVector` _newtrack_0 _newtrack_0 _newtrack_0))
      (`SceneComponent.SetRelativeScale3D` (`self.Collider7`) (`KismetMathLibrary.MakeVector` _newtrack_0 _newtrack_0 _newtrack_0))
      (`SceneComponent.SetRelativeScale3D` (`self.Collider6`) (`KismetMathLibrary.MakeVector` _newtrack_0 _newtrack_0 _newtrack_0))
      (`SceneComponent.SetRelativeScale3D` (`self.Collider5`) (`KismetMathLibrary.MakeVector` _newtrack_0 _newtrack_0 _newtrack_0))
      (`SceneComponent.SetRelativeScale3D` (`self.Collider4`) (`KismetMathLibrary.MakeVector` _newtrack_0 _newtrack_0 _newtrack_0))
      (`SceneComponent.SetRelativeScale3D` (`self.Collider2`) (`KismetMathLibrary.MakeVector` _newtrack_0 _newtrack_0 _newtrack_0))
      (`SceneComponent.SetRelativeScale3D` (`self.Collider3`) (`KismetMathLibrary.MakeVector` _newtrack_0 _newtrack_0 _newtrack_0))
      (`SceneComponent.SetRelativeScale3D` (`self.Collider1`) (`KismetMathLibrary.MakeVector` _newtrack_0 _newtrack_0 _newtrack_0)))
    (:`Finished`
      (`self.K2_DestroyActor`))))

(event `self.ReceiveActorBeginOverlap`
  (params (OtherActor :type "Actor Object Reference"))
  (bind _asbp_player_character (cast `/Game/Blueprints/Actors/BP_PlayerCharacter` OtherActor))
  (`GameplayStatics.ApplyDamage` _asbp_player_character (`self.Damage`)))

(fn `UserConstructionScript`)