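; BP_SporeCloud is an enemy spore hazard that damages the player while they stand inside it.
; On BeginPlay it gives the cloud sphere a dynamic spore material, then a timeline drives its scale and opacity.
; In parallel, an endless delay loop repeatedly checks whether the player pawn overlaps the Sphere and applies SporeDamage with a damage type named for ignoring invincibility.
; The graph never destroys the actor or stops the loop.
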(event `self.ReceiveBeginPlay`
  (bind _returnvalue (`GameplayStatics.GetPlayerPawn` 0))
  (bind _returnvalue_2 (`KismetMaterialLibrary.CreateDynamicMaterialInstance` "/Game/Materials/M_Spore.M_Spore"))
  (bind _output_get (set `self.SporeMatRef` _returnvalue_2))
  (`PrimitiveComponent.SetMaterial` (`self.CloudSphere`) 0 _output_get)
  (`|ExecutionSequence`
    (:`then_0`
      (bind (_direction _lareg _opac) (`Timeline|Spodf` :!via `PlayFromStart`)
        (:`Update`
          (`SceneComponent.SetRelativeScale3D` (`self.CloudSphere`) (`KismetMathLibrary.MakeVector` _lareg _lareg _lareg))
          (`MaterialInstanceDynamic.SetScalarParameterValue` (`self.SporeMatRef`) "SporeOpacity" _opac))))
    (:`then_1`
      (`KismetSystemLibrary.Delay` 0.3 :!label _label)
      (if (`PrimitiveComponent.IsOverlappingActor` (`self.Sphere`) _returnvalue)
        (`GameplayStatics.ApplyDamage` _returnvalue (`self.SporeDamage`) null null "/Game/Blueprints/FrameWork/IgnoreInvincibilityType.IgnoreInvincibilityType_C")
        (goto _label)
        (else
          (goto _label))))))

(fn `UserConstructionScript`)