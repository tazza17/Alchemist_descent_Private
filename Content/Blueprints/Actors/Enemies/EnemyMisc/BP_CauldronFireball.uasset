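; BP_CauldronFireball is an enemy projectile that flies toward the player's position at spawn and damages the player on contact.
; On BeginPlay it rotates to face the player pawn, then moves along its local forward axis by Speed every Tick, without homing or delta-time scaling.
; Overlapping BP_PlayerCharacter with the root sphere applies ProjectileDamage, spawns a particle system, and destroys the actor one tick later.
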(event `self.ReceiveBeginPlay`
  (`self.K2_SetActorRotation` (`KismetMathLibrary.FindLookAtRotation` (`self.K2_GetActorLocation`) (`self.K2_GetActorLocation` (`GameplayStatics.GetPlayerPawn` 0)))))

(event `self.ReceiveTick`
  (params (DeltaSeconds :type "Float (single-precision)"))
  (`self.K2_AddActorLocalOffset` (`KismetMathLibrary.MakeVector` (`self.Speed`))))

(event `self.SphereColRoot.OnComponentBeginOverlap`
  (params (OverlappedComponent :type "PrimitiveComponent Object Reference") (OtherActor :type "Actor Object Reference") (OtherComp :type "PrimitiveComponent Object Reference") (OtherBodyIndex :type Integer) (bFromSweep :type Boolean) (SweepResult :type "HitResult Structure (by ref)"))
  (bind _asbp_player_character (cast `/Game/Blueprints/Actors/BP_PlayerCharacter` OtherActor))
  (`GameplayStatics.ApplyDamage` _asbp_player_character (`self.ProjectileDamage`))
  (`NiagaraFunctionLibrary.SpawnSystemAtLocation` null (`self.K2_GetActorLocation`))
  (`KismetSystemLibrary.DelayUntilNextTick`)
  (`self.K2_DestroyActor`))

(fn `UserConstructionScript`)