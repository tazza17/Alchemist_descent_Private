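; BP_BossWindburst is an enemy windburst actor that knocks the player away on overlapping its sphere.
; The overlap launches BP_PlayerCharacter outward from the actor's center, clamping vertical velocity to a minimum upward lift.
; An overlapping BP_Potion instead gets a much weaker local-space projectile velocity.
; That potion direction reads the failed player cast's location rather than the potion's.
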(event `self.Sphere.OnComponentBeginOverlap`
  (params (OverlappedComponent :type "PrimitiveComponent Object Reference") (OtherActor :type "Actor Object Reference") (OtherComp :type "PrimitiveComponent Object Reference") (OtherBodyIndex :type Integer) (bFromSweep :type Boolean) (SweepResult :type "HitResult Structure (by ref)"))
  (bind _asbp_player_character (cast `/Game/Blueprints/Actors/BP_PlayerCharacter` OtherActor)
    (:`then`
      (bind _returnvalue (`KismetMathLibrary.GetDirectionUnitVector` (`self.K2_GetActorLocation`) (`self.K2_GetActorLocation` _asbp_player_character)))
      (bind (_returnvalue_x _returnvalue_y _returnvalue_z) (`KismetMathLibrary.BreakVector` (* _returnvalue (1500.0 1500.0 1500.0))))
      (`Character.LaunchCharacter` _asbp_player_character (`KismetMathLibrary.MakeVector` _returnvalue_x _returnvalue_y (`KismetMathLibrary.FClamp` _returnvalue_z 300.0 999999.0)) false false))
    (:`CastFailed`
      (bind _asbp_potion (cast `/Game/Blueprints/Actors/Potions/BP_Potion` OtherActor))
      (`ProjectileMovementComponent.SetVelocityInLocalSpace` (`/Game/Blueprints/Actors/Potions/BP_Potion.ProjectileMovement` _asbp_potion) (* _returnvalue (100.0 100.0 100.0))))))

(fn `UserConstructionScript`)