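; Slime enemy that hops toward the player with a squash-and-stretch bounce.
; After a random delay, a looping timeline animates the model's height and scale, feeds movement input toward the player while above a height threshold, and triggers bounce sounds.
; Tick smoothly yaws it toward the player; the frozen state stops turning and the hop loop until thawed.
; Death plays a sound and scale timeline before handing off to the parent enemy logic.
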(event `BeginMovement`
  (bind _enemymodel (`self.EnemyModel`))
  (bind _returnvalue (`SceneComponent.GetRelativeTransform` _enemymodel))
  (`KismetSystemLibrary.Delay` (`KismetMathLibrary.RandomFloatInRange` 0.0 (`self.SlimeJumpDelayMax`)))
  (bind (_direction _jump _squeeshz _squeeshxy) (`Timeline|Jumpin` :!via `PlayFromStart`)
    (:`Update`
      (`SceneComponent.K2_SetRelativeLocation` _enemymodel (`KismetMathLibrary.MakeVector` (.x (.location _returnvalue)) (.y (.location _returnvalue)) _jump) false false)
      (`SceneComponent.SetRelativeScale3D` (`self.EnemyModel`) (`KismetMathLibrary.MakeVector` _squeeshxy _squeeshxy _squeeshz))
      (if (>= _jump -54.0)
        (`PawnMovementComponent.AddInputVector` (`self.CharacterMovement`) (`KismetMathLibrary.GetDirectionUnitVector` (`self.K2_GetActorLocation`) (`self.K2_GetActorLocation` (`GameplayStatics.GetPlayerPawn` 0))) false)))
    (:`Finished`
      (if (not (`self.IsFrozen`))
        (`self.BeginMovement`)))
    (:`SlimeSound`
      (`self.Slime Bounce Sound Effect`))))

(event `Slime Bounce Sound Effect`
  (`GameplayStatics.PlaySoundAtLocation` "/Game/Audio/Slime_Bounce_Cue.Slime_Bounce_Cue" (`self.K2_GetActorLocation`) (struct) 1.0 1.0 0.0 "/Game/Audio/PP_SoundAttenuation300.PP_SoundAttenuation300" null self null))

(event `self.FinishedFrozen`
  (`self.BeginMovement` :!label _label))

(event `self.ReceiveBeginPlay`
  (`parent.ReceiveBeginPlay`)
  (goto _label))

(event `self.EnemyDeath`
  (`GameplayStatics.PlaySoundAtLocation` "/Game/Audio/Slime_Death_Sound_Effect.Slime_Death_Sound_Effect" (`self.K2_GetActorLocation`) (struct) 0.5 1.0 0.0 "/Game/Audio/PP_SoundAttenuation300.PP_SoundAttenuation300" null null null)
  (bind (_direction _smal) (`Timeline|Squish` :!via `PlayFromStart`)
    (:`Update`
      (`self.SetActorScale3D` (`KismetMathLibrary.MakeVector` _smal _smal _smal)))
    (:`Finished`
      (`parent.EnemyDeath`))))

(event `self.ReceiveTick`
  (params (DeltaSeconds :type "Float (single-precision)"))
  (bind (_returnvalue_roll _returnvalue_pitch _returnvalue_yaw) (`KismetMathLibrary.BreakRotator` (`KismetMathLibrary.RLerp` (`self.K2_GetActorRotation`) (`KismetMathLibrary.FindLookAtRotation` (`self.K2_GetActorLocation`) (`self.K2_GetActorLocation` (`GameplayStatics.GetPlayerPawn` 0))) 0.1 true)))
  (`parent.ReceiveTick` 0.0)
  (if (not (`self.IsFrozen`))
    (`self.K2_SetActorRotation` (`KismetMathLibrary.MakeRotator` 0.0 0.0 _returnvalue_yaw))))

(fn `UserConstructionScript`
  (`parent.UserConstructionScript`))