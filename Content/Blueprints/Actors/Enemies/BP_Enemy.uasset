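; Enemy character with health, contact damage to the player, status effects and a chance to drop loot on death.
; AnyDamage respects i-frames unless IgnoreInvincibilityType is used, doubles damage when marked for death, and triggers popups and hit flash.
; ApplyEffectstoEnemy starts or refreshes fire, hellfire, decay, slow and freeze, using self-calling delayed events for damage over time.
; Death notifies GameInstance_PP, drops loot and destroys attached actors.
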(event `self.ReceiveBeginPlay`)

(event `DestroyParticle`
  (params (Component :type "SceneComponent Object Reference") (System :type "NiagaraSystem Object Reference"))
  ; Destroy Particles
  (for _array_element (`SceneComponent.GetChildrenComponents` (`self.ParticleSpawnPoint`) false)
    (bind _asniagara_particle_system_component (cast `NiagaraComponent` _array_element))
    (if (== (`NiagaraComponent.GetAsset` _asniagara_particle_system_component) System)
      (`ActorComponent.SetActive` _array_element false false)
      (`KismetSystemLibrary.Delay` 5.0)
      (`ActorComponent.K2_DestroyComponent` _array_element)
      (`KismetSystemLibrary.PrintString` "we gotem" true true (struct :`G` 1.0 :`B` 0.059491 :`A` 1.0)))))

(event `FireDebuffWeak`
  (params (Component :type "SceneComponent Object Reference") (System :type "NiagaraSystem Object Reference"))
  ;[0.9406 0.3435 0 0.5] Fire Debuff (Weak)
  (if (<= (`self.FireDebuffTimer`) 0.0)
    (`self.DestroyParticle` Component System)
    (else
      (set `self.FireDebuffTimer` (- (`self.FireDebuffTimer`) 1.0))
      (`GameplayStatics.ApplyDamage` self 1.0 null null "/Game/Blueprints/FrameWork/IgnoreInvincibilityType.IgnoreInvincibilityType_C") ; How much damage per hit
      (`KismetSystemLibrary.Delay` 1.0) ; How long it takes per tick of damage
      (`self.FireDebuffWeak` Component System))))

(event `self.ReceiveAnyDamage`
  (params (Damage :type "Float (single-precision)") (DamageType :type "DamageType Object Reference") (InstigatedBy :type "Controller Object Reference") (DamageCauser :type "Actor Object Reference"))
  (bind _returnvalue (* Damage 2.0))
  ;[1 0.2677 0.2677 0.5] Damage and I-Frame Timer
  (cast `/Game/Blueprints/FrameWork/IgnoreInvincibilityType` DamageType
    (:`then`
      (if (`self.MarkedForDeath?`) :!label _label
        (set `self.EnemyHealth` (- (`self.EnemyHealth`) _returnvalue))
        (`self.PopupText` (`KismetTextLibrary.Conv_StringToText` (`KismetStringLibrary.Concat_StrStr` (`KismetTextLibrary.Conv_TextToString` (`KismetTextLibrary.Conv_DoubleToText` _returnvalue "HalfToEven")) "!")) (make `SlateColor` (struct :`R` 0.182141 :`B` 0.390625 :`A` 1.0)))
        (else
          (set `self.EnemyHealth` (- (`self.EnemyHealth`) Damage))
          (`self.PopupText` (`KismetTextLibrary.Conv_DoubleToText` Damage "HalfToEven") (make `SlateColor` (struct :`R` 1.0 :`G` 0.026571 :`B` 0.000103 :`A` 1.0)))))
      (`self.EnemyFlash`)
      (`KismetSystemLibrary.PrintString` (`KismetStringLibrary.Conv_DoubleToString` (`self.EnemyMaxHealth`)))
      (`KismetSystemLibrary.PrintString` "out of:")
      (`KismetSystemLibrary.PrintString` (`KismetStringLibrary.Conv_DoubleToString` (`self.EnemyHealth`)))
      (`KismetSystemLibrary.PrintString` "ouch, now im on:")
      (if (<= (`self.EnemyHealth`) 0.0)
        (`self.EnemyDeath`)))
    (:`CastFailed`
      (if (`self.CanTakeDamage?`)
        (`self.I-FrameTimer`)
        (goto _label)))))

(event `I-FrameTimer`
  ;[1 0.2677 0.2677 0.5] Damage and I-Frame Timer
  (set `self.CanTakeDamage?` false)
  (`KismetSystemLibrary.Delay` (`self.InvincibilityFrames`))
  (set `self.CanTakeDamage?` true))

(event `FireDebuffStrong`
  (params (Component :type "SceneComponent Object Reference") (System :type "NiagaraSystem Object Reference"))
  ;[0.6823 0 0.1155 0.5] Fire Debuff (Strong)
  (if (<= (`self.HellfireDebuffTimer`) 0.0)
    (`self.DestroyParticle` Component System)
    (else
      (set `self.HellfireDebuffTimer` (- (`self.HellfireDebuffTimer`) 1.0))
      (`GameplayStatics.ApplyDamage` self 2.0 null null "/Game/Blueprints/FrameWork/IgnoreInvincibilityType.IgnoreInvincibilityType_C") ; How much damage per hit
      (`KismetSystemLibrary.Delay` 0.5) ; How long it takes per tick of damage
      (`self.FireDebuffStrong` Component System))))

(event `PopupText`
  (params (Text :type Text) (Color :type "SlateColor Structure") (tEffect_fDamage :type Boolean))
  (if tEffect_fDamage
    (bind _returnvalue (`|SpawnActorFromClass` "/Game/Blueprints/Widgets/BP_PopupText.BP_PopupText_C" (`KismetMathLibrary.MakeTransform` (`self.K2_GetActorLocation`)) "AlwaysSpawn" "MultiplyWithRoot" null null))
    (`/Game/Blueprints/Widgets/BP_PopupText.ChangeWidgetsText` _returnvalue Text Color tEffect_fDamage)
    (else
      (bind _returnvalue_2 (`|SpawnActorFromClass` "/Game/Blueprints/Widgets/BP_PopupText.BP_PopupText_C" (`KismetMathLibrary.MakeTransform` (+ (`self.K2_GetActorLocation`) (`KismetMathLibrary.RandomPointInBoundingBox` (0.0 0.0 0.0) (20.0 20.0 20.0)))) "AlwaysSpawn" "MultiplyWithRoot" null null))
      (`/Game/Blueprints/Widgets/BP_PopupText.ChangeWidgetsText` _returnvalue_2 Text Color tEffect_fDamage))))

(event `EnemyDeath`
  ;[0 0 0 0.5] Death Sequence and Checks for any other alive enemies
  (bind _asgame_instance_pp (cast `/Game/Blueprints/FrameWork/GameInstance_PP` (`GameplayStatics.GetGameInstance`)))
  (`/Game/Blueprints/FrameWork/GameInstance_PP.CheckForEnemies` _asgame_instance_pp)
  (`self.DropLoot`)
  (`NiagaraFunctionLibrary.SpawnSystemAtLocation` (`self.DeathParticle`) (`SceneComponent.K2_GetComponentLocation` (`self.ParticleSpawnPoint`)))
  (`KismetSystemLibrary.DelayUntilNextTick`)
  (for _array_element (`self.GetAttachedActors` true)
    (`self.K2_DestroyActor` _array_element))
  (`self.K2_DestroyActor`))

(event `SlownessDebuff`
  (params (Component :type "SceneComponent Object Reference") (System :type "NiagaraSystem Object Reference"))
  ;[0 0.7892 0.8865 0.5] Slowness Debuff
  (set `CharacterMovementComponent.MaxWalkSpeed` (/ (`self.MovementSpeed`) 3.0) (`self.CharacterMovement`))
  (`KismetSystemLibrary.Delay` (`self.SlownessDebuffTimer`))
  (`self.DestroyParticle` Component System)
  (set `CharacterMovementComponent.MaxWalkSpeed` (`self.MovementSpeed`) (`self.CharacterMovement`)))

(event `FrozenDebuff`
  (params (Component :type "SceneComponent Object Reference") (System :type "NiagaraSystem Object Reference"))
  ;[0 0.02105 0.15 0.5] Frozen Debuff
  (set `CharacterMovementComponent.MaxWalkSpeed` 0.0 (`self.CharacterMovement`))
  (set `self.IsFrozen` true)
  (`KismetSystemLibrary.Delay` (`self.FrozenDebuffTimer`))
  (`self.DestroyParticle` Component System)
  (set `CharacterMovementComponent.MaxWalkSpeed` (`self.MovementSpeed`) (`self.CharacterMovement`))
  (set `self.IsFrozen` false)
  (`self.FinishedFrozen`))

(event `EnemyFlash`
  ; Enemy Flash
  (`MeshComponent.SetOverlayMaterial` (`self.EnemyModel`) "/Game/Materials/M_EnemyHit.M_EnemyHit")
  (`MeshComponent.SetOverlayMaterial` (`self.Mesh`) "/Game/Materials/M_EnemyHit.M_EnemyHit")
  (`KismetSystemLibrary.Delay` 0.1)
  (`MeshComponent.SetOverlayMaterial` (`self.EnemyModel`) null)
  (`MeshComponent.SetOverlayMaterial` (`self.Mesh`) null))

(event `FinishedFrozen`)

(event `DecayDebuff`
  ;[0.1059 5.5e-05 0.1823 0.5] Decay Debuff
  (if (not (<= (`self.DecayTimer`) 0.0))
    (set `self.DecayTimer` (- (`self.DecayTimer`) 1.0))
    (`GameplayStatics.ApplyDamage` self 4.0 null null "/Game/Blueprints/FrameWork/IgnoreInvincibilityType.IgnoreInvincibilityType_C") ; How much damage per hit
    (`KismetSystemLibrary.Delay` 1.0) ; How long it takes per tick of damage
    (`self.DecayDebuff`)))

(event `self.ReceiveTick`
  (params (DeltaSeconds :type "Float (single-precision)"))
  (bind _returnvalue (`GameplayStatics.GetPlayerPawn` 0))
  ;[0.01664 0.15 0.01888 0.5] Event Tick
  (if (`PrimitiveComponent.IsOverlappingActor` (`self.AttackCollider`) _returnvalue)
    (bind _asbp_player_character (cast `/Game/Blueprints/Actors/BP_PlayerCharacter` _returnvalue))
    (`GameplayStatics.ApplyDamage` _asbp_player_character (`self.AttackDamage`))))

(event `MarkedForDeath`
  (set `self.MarkedForDeath?` true)
  (`self.ParticleFunction` "/Game/Blueprints/Particles/PS_Marked.PS_Marked")
  (`self.PopupText` "Marked for death..." (make `SlateColor` (struct :`R` 0.579931 :`G` 0.000298 :`B` 1.0 :`A` 1.0))))

(event `/Game/Blueprints/FrameWork/Interface_PP.ApplyEffectsToEnemy`
  (params (AppliedEffect :type "/Game/Blueprints/FrameWork/Enum_PotionEffectsList Enum" :default "NewEnumerator6"))
  ;[0.07428 0.08794 0.15 0.5] Effects Manager
  (switch `/Game/Blueprints/FrameWork/Enum_PotionEffectsList` AppliedEffect
    (:`NewEnumerator0`
      (bind (_returnvalue _systemref) (`self.ParticleFunction` "/Game/Blueprints/Particles/PS_Fire.PS_Fire"))
      (if (> (`self.FireDebuffTimer`) 0.0)
        (set `self.FireDebuffTimer` 5.0)
        (else
          (set `self.FireDebuffTimer` 5.0)
          (`self.FireDebuffWeak` _returnvalue _systemref)
          (`self.PopupText` "On Fire!" (make `SlateColor` (struct :`R` 0.682292 :`G` 0.082203 :`A` 1.0)) true))))
    (:`NewEnumerator1`
      (bind (_returnvalue_2 _systemref_2) (`self.ParticleFunction` "/Game/Blueprints/Particles/PS_HellFire.PS_HellFire"))
      (if (> (`self.HellfireDebuffTimer`) 0.0)
        (set `self.HellfireDebuffTimer` 8.0)
        (else
          (set `self.HellfireDebuffTimer` 8.0)
          (`self.FireDebuffStrong` _returnvalue_2 _systemref_2)
          (`self.PopupText` "On Hellfire!" (make `SlateColor` (struct :`R` 0.328125 :`B` 0.079879 :`A` 1.0)) true))))
    (:`NewEnumerator2`
      (bind (_returnvalue_3 _systemref_3) (`self.ParticleFunction` "/Game/Blueprints/Particles/PS_Snow.PS_Snow"))
      (if (> (`self.SlownessDebuffTimer`) 0.0)
        (set `self.SlownessDebuffTimer` 5.0)
        (else
          (set `self.SlownessDebuffTimer` 5.0)
          (`self.SlownessDebuff` _returnvalue_3 _systemref_3)
          (`self.PopupText` "Chilled!" (make `SlateColor` (struct :`R` 0.192985 :`G` 0.492198 :`B` 0.869792 :`A` 1.0)) true)))
      (bind _returnvalue_4 (`|SpawnActorFromClass` "/Game/Blueprints/Widgets/BP_Chilling.BP_Chilling_C" (`KismetMathLibrary.MakeTransform` (`self.K2_GetActorLocation`)) "AlwaysSpawn" "MultiplyWithRoot" null null))
      (`self.K2_AttachToComponent` _returnvalue_4 (`self.ParticleSpawnPoint`) "None" "SnapToTarget" "KeepRelative" "KeepRelative" true))
    (:`NewEnumerator3`
      (bind (_returnvalue_5 _systemref_4) (`self.ParticleFunction` "/Game/Blueprints/Particles/PS_Snow.PS_Snow"))
      (if (> (`self.FrozenDebuffTimer`) 0.0)
        (set `self.FrozenDebuffTimer` 4.0)
        (else
          (set `self.FrozenDebuffTimer` 4.0)
          (`self.FrozenDebuff` _returnvalue_5 _systemref_4)
          (`self.PopupText` "Frozen!" (make `SlateColor` (struct :`G` 0.384531 :`B` 0.869792 :`A` 1.0)) true)))
      (bind _returnvalue_6 (`|SpawnActorFromClass` "/Game/Blueprints/Widgets/BP_Freezing.BP_Freezing_C" (`KismetMathLibrary.MakeTransform` (`self.K2_GetActorLocation`)) "AlwaysSpawn" "MultiplyWithRoot" null null))
      (`self.K2_AttachToComponent` _returnvalue_6 (`self.ParticleSpawnPoint`) "None" "SnapToTarget" "KeepRelative" "KeepRelative" true))
    (:`NewEnumerator4`
      (if (> (`self.DecayTimer`) 0.0)
        (set `self.DecayTimer` 5.0)
        (else
          (set `self.DecayTimer` 5.0)
          (`self.DecayDebuff`)
          (`self.PopupText` "Decaying!" (make `SlateColor` (struct :`A` 1.0)) true)))
      (bind _returnvalue_7 (`|SpawnActorFromClass` "/Game/Blueprints/Widgets/BP_Decaying.BP_Decaying_C" (`KismetMathLibrary.MakeTransform` (`self.K2_GetActorLocation`)) "AlwaysSpawn" "MultiplyWithRoot" null null))
      (`self.K2_AttachToComponent` _returnvalue_7 (`self.ParticleSpawnPoint`) "None" "SnapToTarget" "KeepRelative" "KeepRelative" true))))

(fn `CheckForSpaceHUD`
  (returns (`AnySpace?` :type Boolean) (EmptySlot :type "/Game/Blueprints/Widgets/WBP_HotbarSlot Object Reference"))
  (return false null))

(fn `ChooseRandomEnemy`
  (params (AlreadySelectedEnemy :type "/Game/Blueprints/Actors/Enemies/BP_Enemy Class Reference"))
  (returns (ChosenEnemy :type "/Game/Blueprints/Actors/Enemies/BP_Enemy Class Reference") (SpawnModifiers :type "/Game/Blueprints/FrameWork/S_EnemyModifiers Structure"))
  (return null))

(fn `DropLoot`
  (bind (_returnvalue_x _returnvalue_y _returnvalue_z) (`KismetMathLibrary.BreakVector` (`self.K2_GetActorLocation`)))
  (if (`KismetMathLibrary.RandomBoolWithWeight` (`self.LootDropChance`))
    (`|SpawnActorFromClass` (`KismetArrayLibrary.Array_Random` (`self.Lootpool`)) (`KismetMathLibrary.MakeTransform` (`KismetMathLibrary.MakeVector` _returnvalue_x _returnvalue_y (+ _returnvalue_z 20.0))) "Undefined" "MultiplyWithRoot" null null)))

(fn `GetChestItem`
  (params (Rarity :type Integer))
  (returns (ItemReceived :type "/Game/Blueprints/Actors/Interactables/Pickups/BP_PickUp Class Reference"))
  (return null))

(fn `GetPlayerStats`
  (returns (PlayerStats :type "/Game/Blueprints/FrameWork/S_PlayerStats Structure") (CurrentTime :type "Float (double-precision)"))
  (return (struct) 0.0))

(fn `GetRandomLevel`
  (params (LevelType :type "/Game/Blueprints/FrameWork/Enum_PortalTypes Enum" :default "NewEnumerator0"))
  (returns (ChosenLevel :type Name))
  (return "None"))

(fn `ParticleFunction`
  (params (SystemTemplate :type "NiagaraSystem Object Reference"))
  (returns (ReturnValue :type "SceneComponent Object Reference") (SystemRef :type "NiagaraSystem Object Reference"))
  (bind _particlespawnpoint (`self.ParticleSpawnPoint`))
  (bind _returnvalue (`NiagaraFunctionLibrary.SpawnSystemAttached` SystemTemplate _particlespawnpoint "None" (`SceneComponent.K2_GetComponentLocation` _particlespawnpoint) (struct) "KeepWorldPosition"))
  (return _returnvalue (`NiagaraComponent.GetAsset` _returnvalue)))

(fn `UserConstructionScript`
  (set `self.EnemyHealth` (`self.EnemyMaxHealth`))
  (set `CharacterMovementComponent.MaxWalkSpeed` (`self.MovementSpeed`) (`self.CharacterMovement`)))