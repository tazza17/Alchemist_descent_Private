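; Evil cauldron enemy that watches the player and launches fireballs while it has line of sight and is not frozen.
; Tick turns the eye toward the camera, eases the bone's yaw toward the player, and updates CanSeePlayer with a visibility trace.
; Timelines drive idle bobbing, symbol spin and the magic-orb charge.
; A self-repeating event rechecks conditions after each charge, then spawns BP_CauldronFireball with the enemy's AttackDamage.
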(event `self.ReceiveTick`
  (params (DeltaSeconds :type "Float (single-precision)"))
  (bind _bone (`self.Bone`))
  (bind _eye (`self.Eye`))
  (bind (_relativerotation_roll _relativerotation_pitch _relativerotation_yaw) (`KismetMathLibrary.BreakRotator` (`SceneComponent.RelativeRotation` _bone)))
  (bind (_returnvalue_roll _returnvalue_pitch _returnvalue_yaw) (`KismetMathLibrary.BreakRotator` (`KismetMathLibrary.FindLookAtRotation` (`self.K2_GetActorLocation`) (`self.K2_GetActorLocation` (`GameplayStatics.GetPlayerPawn` 0)))))
  (bind (_returnvalue_roll_2 _returnvalue_pitch_2 _returnvalue_yaw_2) (`KismetMathLibrary.BreakRotator` (`KismetMathLibrary.RLerp` (`KismetMathLibrary.MakeRotator` 0.0 0.0 _relativerotation_yaw) (`KismetMathLibrary.MakeRotator` 0.0 0.0 _returnvalue_yaw) 0.1 true)))
  (bind (_returnvalue_roll_3 _returnvalue_pitch_3 _returnvalue_yaw_3) (`KismetMathLibrary.BreakRotator` (`KismetMathLibrary.FindLookAtRotation` (`SceneComponent.K2_GetComponentLocation` _eye) (`SceneComponent.K2_GetComponentLocation` (`self.GetComponentByClass` (`GameplayStatics.GetPlayerPawn` 0) "/Script/Engine.CameraComponent")))))
  ; Rotations
  (`parent.ReceiveTick` DeltaSeconds)
  (`SceneComponent.K2_SetRelativeRotation` _eye (`KismetMathLibrary.MakeRotator` _returnvalue_roll_3 _returnvalue_pitch_3 _returnvalue_yaw_3) false false)
  (`SceneComponent.K2_SetRelativeRotation` _bone (`KismetMathLibrary.MakeRotator` 0.0 0.0 _returnvalue_yaw_2) false false)
  (`SceneComponent.K2_SetRelativeRotation` (`self.MagicOrb`) (`KismetMathLibrary.RandomRotator` false) false false)
  (bind _outhit (`KismetSystemLibrary.LineTraceSingle` :`Start` (`SceneComponent.K2_GetComponentLocation` (`self.Eye`)) :`End` (`self.K2_GetActorLocation` (`GameplayStatics.GetPlayerPawn` 0)) :`TraceChannel` "TraceTypeQuery1" :`DrawDebugType` "ForOneFrame"))
  (if (`GameplayStatics.BreakHitResult` _outhit)
    (set `self.CanSeePlayer` false)
    (else
      (set `self.CanSeePlayer` true))))

(event `self.ReceiveBeginPlay`
  (`parent.ReceiveBeginPlay`)
  (`|ExecutionSequence`
    (:`then_0`
      ; PerpetualAnimations
      (bind (_direction _upanddown _symbolrotation) (`Timeline|Animations`)
        (:`Update`
          (`SceneComponent.K2_SetRelativeLocation` (`self.Bone`) (`KismetMathLibrary.MakeVector` 0.0 0.0 _upanddown) false false)
          (`SceneComponent.K2_SetRelativeRotation` (`self.Symbol`) (`KismetMathLibrary.MakeRotator` 0.0 0.0 _symbolrotation) false false))))
    (:`then_1`
      (`self.SpawnFireball`))))

(event `SpawnFireball`
  (bind _magicorb (`self.MagicOrb`))
  ;[0.15 0.0541 0.149 0.5] Spawn Fireball
  (if (and (`self.CanSeePlayer`) (!= (`self.IsFrozen`) true))
    (`SceneComponent.SetVisibility` _magicorb true false)
    (bind (_direction _flaoting) (`Timeline|Magic` :!via `PlayFromStart`)
      (:`Update`
        (`SceneComponent.K2_SetRelativeLocation` _magicorb (`KismetMathLibrary.MakeVector` 0.0 0.0 _flaoting) false false))
      (:`Finished`
        (`SceneComponent.SetVisibility` _magicorb false false)
        (if (and (`self.CanSeePlayer`) (!= (`self.IsFrozen`) true))
          (bind _returnvalue (`|SpawnActorFromClass` "/Game/Blueprints/Actors/Enemies/EnemyMisc/BP_CauldronFireball.BP_CauldronFireball_C" (`KismetMathLibrary.MakeTransform` (`SceneComponent.K2_GetComponentLocation` _magicorb)) "AlwaysSpawn" "MultiplyWithRoot" null null))
          (set `/Game/Blueprints/Actors/Enemies/EnemyMisc/BP_CauldronFireball.ProjectileDamage` (`self.AttackDamage`) _returnvalue)
          (`KismetSystemLibrary.Delay` 0.5)
          (`self.SpawnFireball`)
          (else
            (`KismetSystemLibrary.Delay` 0.2)
            (`self.SpawnFireball`)))))
    (else
      (`KismetSystemLibrary.Delay` 0.2)
      (`self.SpawnFireball`))))

(fn `UserConstructionScript`
  (`parent.UserConstructionScript`))