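; Pumpkin enemy that chases the player pawn and periodically switches a rolling rotation on and off.
; A looping timer flips IsRolling and toggles the RotatingMovement component's tick to start or stop the spin.
; Each tick, unless frozen, it eases its yaw toward the player and feeds CharacterMovement input along the direction to them, after running the parent tick.
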(event `self.ReceiveBeginPlay`
  (`KismetSystemLibrary.K2_SetTimer` null "ToggleRoll" 2.0 true))

(event `ToggleRoll`
  (if (`self.IsRolling`)
    (`ActorComponent.SetComponentTickEnabled` (`self.RotatingMovement`) (stale _output_get))
    (bind _output_get (set `self.IsRolling` false))
    (else
      (`ActorComponent.SetComponentTickEnabled` (`self.RotatingMovement`) (stale _output_get_2))
      (bind _output_get_2 (set `self.IsRolling` true)))))

(event `self.ReceiveTick`
  (params (DeltaSeconds :type "Float (single-precision)"))
  (bind (_returnvalue_roll _returnvalue_pitch _returnvalue_yaw) (`KismetMathLibrary.BreakRotator` (`KismetMathLibrary.RLerp` (`self.K2_GetActorRotation`) (`KismetMathLibrary.FindLookAtRotation` (`self.K2_GetActorLocation`) (`self.K2_GetActorLocation` (`GameplayStatics.GetPlayerPawn` 0))) 0.1 true)))
  (`parent.ReceiveTick` 0.0)
  (if (not (`self.IsFrozen`))
    (`self.K2_SetActorRotation` (`KismetMathLibrary.MakeRotator` 0.0 0.0 _returnvalue_yaw))
    (`PawnMovementComponent.AddInputVector` (`self.CharacterMovement`) (`KismetMathLibrary.GetDirectionUnitVector` (`self.K2_GetActorLocation`) (`self.K2_GetActorLocation` (`GameplayStatics.GetPlayerPawn` 0))) false)))

(fn `UserConstructionScript`
  (`parent.UserConstructionScript`))