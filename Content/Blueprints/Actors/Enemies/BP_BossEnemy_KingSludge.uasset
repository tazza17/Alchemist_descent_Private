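; King Sludge, a slime boss with a health bar that turns to face the player and hops toward them, pausing when frozen.
; After one or two hops it picks a random fire, ice, earth, wind or lightning attack, tints its dynamic material, then resumes hopping.
; Timelines drive squash-and-stretch and most attack spawns, while lightning repeats strikes around the player on a delay loop.
; Death shrinks it and leaves a regular slime.
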(event `self.EnemyDeath`
  (bind _particlespawnpoint (`self.ParticleSpawnPoint`))
  (bind _returnvalue (`SceneComponent.K2_GetComponentLocation` _particlespawnpoint))
  ;[0.15 1.2e-05 0.002895 0.5] Death Sequence
  (`PlayerController.ClientStartCameraShake` :`self` (`GameplayStatics.GetPlayerController` 0) :`Shake` "/Game/Blueprints/FrameWork/BP_CameraShakeSlimeBossDeath.BP_CameraShakeSlimeBossDeath_C")
  (`NiagaraFunctionLibrary.SpawnSystemAttached` "/Game/Blueprints/Particles/PS_SlimeBossDeath1.PS_SlimeBossDeath1" _particlespawnpoint "None" (0.0 0.0 0.0) (struct) "KeepRelativeOffset")
  (`/Game/Blueprints/Widgets/WBP_BossHealthbar.DeathSequence` (`self.BossBarRef`))
  (`KismetSystemLibrary.Delay` 3.0)
  (bind (_direction _squeeze) (`Timeline|ScaleSmall`)
    (:`Update`
      (`self.SetActorScale3D` (`KismetMathLibrary.MakeVector` _squeeze _squeeze _squeeze)))
    (:`Finished`
      (`NiagaraFunctionLibrary.SpawnSystemAtLocation` "/Game/Blueprints/Particles/PS_SlimeBossDeath2.PS_SlimeBossDeath2" _returnvalue)
      (`|SpawnActorFromClass` "/Game/Blueprints/Actors/Enemies/BP_Enemy_Slime.BP_Enemy_Slime_C" (`KismetMathLibrary.MakeTransform` _returnvalue) "AlwaysSpawn" "MultiplyWithRoot" null null)
      (`KismetSystemLibrary.DelayUntilNextTick`)
      (for _array_element (`self.GetAttachedActors` true)
        (`self.K2_DestroyActor` _array_element))
      (`self.K2_DestroyActor`))))

(event `ChooseNewAttack`
  (switch `int` (`KismetMathLibrary.RandomIntegerInRange` 0 4)
    (:`Default`
      (`self.FireAttack` :!label _label)
      (`KismetSystemLibrary.PrintString` "Fire Attack CRAACKEL" true true (struct :`R` 1.0 :`G` 0.21169 :`A` 1.0)))
    (:`0`
      (goto _label))
    (:`1`
      (`self.IceAttack`)
      (`KismetSystemLibrary.PrintString` "Ice Attack BRRR" true true (struct :`G` 0.395262 :`B` 1.0 :`A` 1.0)))
    (:`2`
      (`self.EarthAttack`)
      (`KismetSystemLibrary.PrintString` "Stone Attack CRACK" true true (struct :`R` 1.0 :`G` 0.21169 :`A` 1.0)))
    (:`3`
      (`self.WindAttack`)
      (`KismetSystemLibrary.PrintString` "Wind Attack WOOSH" true true (struct :`R` 1.0 :`G` 0.21169 :`A` 1.0)))
    (:`4`
      (`self.LightningAttack`)
      (`KismetSystemLibrary.PrintString` "Lightning Attack ZAP" true true (struct :`R` 1.0 :`G` 0.21169 :`A` 1.0)))))

(event `RegularJump`
  ; Jumping
  (set `self.JumpCount` (`KismetMathLibrary.RandomIntegerInRange` 1 2))
  (`self.JumpLoop`))

(event `FireAttack`
  ;[0.9323 0.1652 0 0.5] FireAttack
  (`self.SwitchToColour` (struct :`R` 1.0 :`G` 0.020553 :`B` 8.1e-05 :`A` 1.0))
  (bind (_direction _scalez _scalexy) (`Timeline|SqueeshFire` :!via `PlayFromStart`)
    (:`Update`
      (`SceneComponent.SetRelativeScale3D` (`self.EnemyModel`) (`KismetMathLibrary.MakeVector` _scalexy _scalexy _scalez)))
    (:`Finished`
      (`self.FinishedAttack`))
    (:`ShootFireballs`
      (for _ (range (+ (`KismetMathLibrary.RandomIntegerInRange` 10 15) 1))
        (bind _returnvalue (`|SpawnActorFromClass` "/Game/Blueprints/Actors/Enemies/EnemyMisc/BP_BossFireball.BP_BossFireball_C" (`KismetMathLibrary.MakeTransform` (`self.K2_GetActorLocation`) (`KismetMathLibrary.MakeRotator` (`KismetMathLibrary.RandomFloatInRange` -40.0 -70.0) (`KismetMathLibrary.RandomFloatInRange` 40.0 70.0) (`KismetMathLibrary.RandomFloatInRange` 0.0 360.0))) "AlwaysSpawn" "MultiplyWithRoot" null null))
        (set `/Game/Blueprints/Actors/Enemies/EnemyMisc/BP_BossFireball.Damage` (`self.AttackDamage`) _returnvalue)))))

(event `JumpLoop`
  (bind _enemymodel (`self.EnemyModel`))
  (bind _returnvalue (`SceneComponent.GetRelativeTransform` _enemymodel))
  ; Jumping
  (if (<= (`self.JumpCount`) 0)
    (`self.ChooseNewAttack`)
    (else
      (`KismetSystemLibrary.Delay` (`KismetMathLibrary.RandomFloatInRange` 0.2 (`self.SlimeJumpDelayMax`)))
      (bind (_direction _jump _squeeshz _squeeshxy) (`Timeline|Jumpin` :!via `PlayFromStart`)
        (:`Update`
          (`SceneComponent.K2_SetRelativeLocation` _enemymodel (`KismetMathLibrary.MakeVector` (.x (.location _returnvalue)) (.y (.location _returnvalue)) _jump) false false)
          (`SceneComponent.SetRelativeScale3D` (`self.EnemyModel`) (`KismetMathLibrary.MakeVector` _squeeshxy _squeeshxy _squeeshz))
          (if (>= _jump -54.0)
            (`PawnMovementComponent.AddInputVector` (`self.CharacterMovement`) (`KismetMathLibrary.GetDirectionUnitVector` (`self.K2_GetActorLocation`) (`self.K2_GetActorLocation` (`GameplayStatics.GetPlayerPawn` 0))) false)))
        (:`Finished`
          (if (not (`self.IsFrozen`))
            (set `self.JumpCount` (- (`self.JumpCount`) 1))
            (`self.JumpLoop`)))
        (:`Shake`
          (`PlayerController.ClientStartCameraShake` :`self` (`GameplayStatics.GetPlayerController` 0) :`Shake` "/Game/Blueprints/FrameWork/BP_CameraShakeExplosion.BP_CameraShakeExplosion_C"))))))

(event `IceAttack`
  (bind (_returnvalue_x _returnvalue_y _returnvalue_z) (`KismetMathLibrary.BreakVector` (`self.K2_GetActorLocation`)))
  ;[0.008742 0.4004 0.8323 0.5] Ice Attack
  (`self.SwitchToColour` (struct :`R` 0.036647 :`G` 0.455991 :`B` 1.0 :`A` 1.0))
  (bind (_direction _squishz _squishxy) (`Timeline|SqueeshIce` :!via `PlayFromStart`)
    (:`Update`
      (`SceneComponent.SetRelativeScale3D` (`self.EnemyModel`) (`KismetMathLibrary.MakeVector` _squishxy _squishxy _squishz)))
    (:`Finished`
      (`self.FinishedAttack`))
    (:`IceShoot`
      (set `self.IcicleRotation` 0.0)
      (for _ (range 31)
        (bind _returnvalue (`|SpawnActorFromClass` "/Game/Blueprints/Actors/Enemies/EnemyMisc/BP_BossIcicle.BP_BossIcicle_C" (`KismetMathLibrary.MakeTransform` (`KismetMathLibrary.MakeVector` _returnvalue_x _returnvalue_y (- _returnvalue_z 80.0)) (`KismetMathLibrary.MakeRotator` 0.0 0.0 (`self.IcicleRotation`))) "AlwaysSpawn" "MultiplyWithRoot" null null))
        (set `/Game/Blueprints/Actors/Enemies/EnemyMisc/BP_BossIcicle.Damage` (/ (`self.AttackDamage`) 1.5) _returnvalue)
        (set `self.IcicleRotation` (+ (`self.IcicleRotation`) 12.0))))))

(event `FinishedAttack`
  (`self.SwitchToColour` (struct :`G` 1.0 :`A` 1.0))
  (`KismetSystemLibrary.Delay` 1.0)
  (`self.RegularJump`))

(event `self.FinishedFrozen`
  (`self.JumpLoop`))

(event `self.ReceiveTick`
  (params (DeltaSeconds :type "Float (single-precision)"))
  (bind (_relativelocation_x _relativelocation_y _relativelocation_z) (`KismetMathLibrary.BreakVector` (`SceneComponent.RelativeLocation` (`self.EnemyModel`))))
  (bind (_returnvalue_roll _returnvalue_pitch _returnvalue_yaw) (`KismetMathLibrary.BreakRotator` (`KismetMathLibrary.RLerp` (`self.K2_GetActorRotation`) (`KismetMathLibrary.FindLookAtRotation` (`self.K2_GetActorLocation`) (`self.K2_GetActorLocation` (`GameplayStatics.GetPlayerPawn` 0))) 0.05 true)))
  ; Rotation
  (`parent.ReceiveTick` 0.0)
  (if (<= _relativelocation_z 53.0)
    (set `self.OnFloor` true)
    (else
      (set `self.OnFloor` false)))
  (if (not (`self.IsFrozen`))
    (`self.K2_SetActorRotation` (`KismetMathLibrary.MakeRotator` 0.0 0.0 _returnvalue_yaw))))

(event `EarthAttack`
  (bind (_returnvalue_x _returnvalue_y _returnvalue_z) (`KismetMathLibrary.BreakVector` (`self.K2_GetActorLocation`)))
  (bind _enemymodel (`self.EnemyModel`))
  (bind _returnvalue (`SceneComponent.GetRelativeTransform` _enemymodel))
  ;[0.15 0.05933 0.01703 0.5] Earth Attack
  (`self.SwitchToColour` (struct :`R` 0.165625 :`G` 0.105691 :`B` 0.041554 :`A` 1.0))
  (bind (_direction _megajump _squishz _squishxy) (`Timeline|SqueeshEarth` :!via `PlayFromStart`)
    (:`Update`
      (`SceneComponent.K2_SetRelativeLocation` _enemymodel (`KismetMathLibrary.MakeVector` (.x (.location _returnvalue)) (.y (.location _returnvalue)) _megajump) false false)
      (`SceneComponent.SetRelativeScale3D` (`self.EnemyModel`) (`KismetMathLibrary.MakeVector` _squishxy _squishxy _squishz)))
    (:`Finished`
      (`self.FinishedAttack`))
    (:`RockSpawn`
      (bind _returnvalue_2 (`|SpawnActorFromClass` "/Game/Blueprints/Actors/Enemies/EnemyMisc/BP_BossStoneCircle.BP_BossStoneCircle_C" (`KismetMathLibrary.MakeTransform` (`KismetMathLibrary.MakeVector` _returnvalue_x _returnvalue_y (- _returnvalue_z 150.0))) "AlwaysSpawn" "MultiplyWithRoot" null null))
      (set `/Game/Blueprints/Actors/Enemies/EnemyMisc/BP_BossStoneCircle.Damage` (* (`self.AttackDamage`) 1.5) _returnvalue_2))))

(event `self.ReceiveBeginPlay`
  ; BeginPlay
  (`parent.ReceiveBeginPlay`)
  (bind _returnvalue (`PrimitiveComponent.CreateDynamicMaterialInstance` (`self.EnemyModel`) 2 "/Game/Materials/M_SlimeBoss_BaseDynamic.M_SlimeBoss_BaseDynamic" "None"))
  (bind _output_get (set `self.MatRef` _returnvalue))
  (`MaterialInstanceDynamic.SetVectorParameterValue` _output_get (`self.ParamName`) (struct :`G` 1.0 :`A` 1.0))
  (bind _returnvalue_2 (`|CreateWidget` "/Game/Blueprints/Widgets/WBP_BossHealthbar.WBP_BossHealthbar_C"))
  (`UserWidget.AddToViewport` _returnvalue_2 0)
  (`/Game/Blueprints/Widgets/WBP_BossHealthbar.SetStats` _returnvalue_2 self "King Sludge")
  (set `self.BossBarRef` _returnvalue_2)
  (`self.RegularJump`))

(event `SwitchToColour`
  (params (LinCol :type "LinearColor Structure"))
  (bind _matref (`self.MatRef`))
  (bind _paramname (`self.ParamName`))
  ; Switch to Colour
  (`Timeline|Switch` :!via `PlayFromStart`
    (:`Update`
      (bind _returnvalue (`MaterialInstanceDynamic.K2_GetVectorParameterValue` _matref _paramname))
      (`MaterialInstanceDynamic.SetVectorParameterValue` _matref _paramname (`KismetMathLibrary.LinearColorLerp` _returnvalue LinCol 0.03)))))

(event `WindAttack`
  ;[0.6157 0.7618 0.7906 0.5] Wind Attack
  (`self.SwitchToColour` (struct :`R` 0.636478 :`G` 0.981371 :`B` 1.0 :`A` 1.0))
  (bind (_direction _scalez _scalexy) (`Timeline|WindTImeline` :!via `PlayFromStart`)
    (:`Update`
      (`SceneComponent.SetRelativeScale3D` (`self.EnemyModel`) (`KismetMathLibrary.MakeVector` _scalexy _scalexy _scalez)))
    (:`Finished`
      (`self.FinishedAttack`))
    (:`WindBurst`
      (`|SpawnActorFromClass` "/Game/Blueprints/Actors/Enemies/EnemyMisc/BP_BossWindburst.BP_BossWindburst_C" (`KismetMathLibrary.MakeTransform` (`self.K2_GetActorLocation`)) "AlwaysSpawn" "MultiplyWithRoot" null null))))

(event `LightningAttack`
  (bind (_returnvalue_x _returnvalue_y _returnvalue_z) (`KismetMathLibrary.BreakVector` (`self.K2_GetActorLocation`)))
  (bind (_returnvalue_x_2 _returnvalue_y_2) (`KismetMathLibrary.BreakVector` (`self.K2_GetActorLocation` (`GameplayStatics.GetPlayerPawn` 0))))
  ;[1 0.7048 0.002357 0.5] Lightning Attack
  (`self.SwitchToColour` (struct :`R` 1.0 :`G` 0.795729 :`A` 1.0))
  (set `self.LightningCount` (`KismetMathLibrary.RandomIntegerInRange` 5 10))
  (bind _returnvalue (`NiagaraFunctionLibrary.SpawnSystemAttached` "/Game/Blueprints/Particles/PS_BossLightningChargeup.PS_BossLightningChargeup" (`self.ParticleSpawnPoint`) "None" (0.0 0.0 0.0) (struct) "KeepRelativeOffset"))
  (bind _returnvalue_2 (`|SpawnActorFromClass` "/Game/Blueprints/Actors/Enemies/EnemyMisc/BP_BossLightning.BP_BossLightning_C" (`KismetMathLibrary.MakeTransform` (`KismetMathLibrary.MakeVector` (+ _returnvalue_x_2 (`KismetMathLibrary.RandomFloatInRange` -600.0 600.0)) (+ _returnvalue_y_2 (`KismetMathLibrary.RandomFloatInRange` -600.0 600.0)) (- _returnvalue_z 155.0))) "AlwaysSpawn" "MultiplyWithRoot" null null :!label _label_2))
  (set `/Game/Blueprints/Actors/Enemies/EnemyMisc/BP_BossLightning.LightningDamage` (`self.AttackDamage`) _returnvalue_2)
  (`KismetSystemLibrary.Delay` 0.1)
  (if (<= (`self.LightningCount`) 0)
    (`KismetSystemLibrary.Delay` 2.0)
    (`ActorComponent.K2_DestroyComponent` _returnvalue)
    (`self.FinishedAttack`)
    (else
      (set `self.LightningCount` (- (`self.LightningCount`) 1))
      (goto _label_2))))

(fn `UserConstructionScript`
  (`parent.UserConstructionScript`))