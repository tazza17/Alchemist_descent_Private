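; Mushroom enemy that chases the player and self-destructs into a damaging spore cloud.
; Each tick a visibility line trace gates smoothed turning and movement toward the player until it starts exploding.
; Player overlap with the attack collider plays a scale-up timeline, then spawns BP_SporeCloud with its attack damage, calls the game instance's enemy check and destroys itself with attached actors.
; The construction script picks a random color material.
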(event `self.ReceiveTick`
  (params (DeltaSeconds :type "Float (single-precision)"))
  (bind (_returnvalue_roll _returnvalue_pitch _returnvalue_yaw) (`KismetMathLibrary.BreakRotator` (`KismetMathLibrary.FindLookAtRotation` (`self.K2_GetActorLocation`) (`self.K2_GetActorLocation` (`GameplayStatics.GetPlayerPawn` 0)))))
  (bind (_returnvalue_roll_2 _returnvalue_pitch_2 _returnvalue_yaw_2) (`KismetMathLibrary.BreakRotator` (`KismetMathLibrary.RLerp` (`self.K2_GetActorRotation`) (`KismetMathLibrary.MakeRotator` 0.0 0.0 _returnvalue_yaw) 0.1 true)))
  ; Movement
  (`|ExecutionSequence`
    (:`then_0`
      (bind _outhit (`KismetSystemLibrary.LineTraceSingle` :`Start` (`self.K2_GetActorLocation`) :`End` (`self.K2_GetActorLocation` (`GameplayStatics.GetPlayerPawn` 0)) :`TraceChannel` "TraceTypeQuery1" :`DrawDebugType` "ForOneFrame"))
      (if (`GameplayStatics.BreakHitResult` _outhit)
        (set `self.CanSeePlayer?` false)
        (else
          (set `self.CanSeePlayer?` true))))
    (:`then_1`
      (if (`self.CanSeePlayer?`)
        (if (not (`self.Exploding`))
          (`self.K2_SetActorRotation` (`KismetMathLibrary.MakeRotator` 0.0 0.0 _returnvalue_yaw_2))
          (`PawnMovementComponent.AddInputVector` (`self.CharacterMovement`) (`KismetMathLibrary.GetDirectionUnitVector` (`self.K2_GetActorLocation`) (`self.K2_GetActorLocation` (`GameplayStatics.GetPlayerPawn` 0))) false))))))

(event `self.AttackCollider.OnComponentBeginOverlap`
  (params (OverlappedComponent :type "PrimitiveComponent Object Reference") (OtherActor :type "Actor Object Reference") (OtherComp :type "PrimitiveComponent Object Reference") (OtherBodyIndex :type Integer) (bFromSweep :type Boolean) (SweepResult :type "HitResult Structure (by ref)"))
  ;[0.9156 0.696 0.07726 0.5] Explode
  (cast `/Game/Blueprints/Actors/BP_PlayerCharacter` OtherActor)
  (set `self.Exploding` true)
  (bind (_direction _scaling) (`Timeline|Puffup`)
    (:`Update`
      (`self.SetActorScale3D` (`KismetMathLibrary.MakeVector` _scaling _scaling _scaling)))
    (:`Finished`
      (bind _returnvalue (`|SpawnActorFromClass` "/Game/Blueprints/Actors/Enemies/EnemyMisc/BP_SporeCloud.BP_SporeCloud_C" (`KismetMathLibrary.MakeTransform` (`self.K2_GetActorLocation`)) "AlwaysSpawn" "MultiplyWithRoot" null null))
      (set `/Game/Blueprints/Actors/Enemies/EnemyMisc/BP_SporeCloud.SporeDamage` (`self.AttackDamage`) _returnvalue)
      (bind _asgame_instance_pp (cast `/Game/Blueprints/FrameWork/GameInstance_PP` (`GameplayStatics.GetGameInstance`)))
      (`/Game/Blueprints/FrameWork/GameInstance_PP.CheckForEnemies` _asgame_instance_pp)
      (`KismetSystemLibrary.DelayUntilNextTick`)
      (for _array_element (`self.GetAttachedActors` true)
        (`self.K2_DestroyActor` _array_element))
      (`self.K2_DestroyActor`))))

(fn `UserConstructionScript`
  (bind _mesh (`self.Mesh`))
  (`parent.UserConstructionScript`)
  (switch `int` (`KismetMathLibrary.RandomIntegerInRange` 0 3)
    (:`0`
      (`PrimitiveComponent.SetMaterial` _mesh 0 "/Game/Materials/M_Mushroom_Enemy_Blue.M_Mushroom_Enemy_Blue"))
    (:`1`
      (`PrimitiveComponent.SetMaterial` _mesh 0 "/Game/Materials/M_Mushroom_Enemy_Red.M_Mushroom_Enemy_Red"))
    (:`2`
      (`PrimitiveComponent.SetMaterial` _mesh 0 "/Game/Materials/M_Mushroom_Enemy_Yellow.M_Mushroom_Enemy_Yellow"))
    (:`3`
      (`PrimitiveComponent.SetMaterial` _mesh 0 "/Game/Materials/M_Mushroom_EnemyPink.M_Mushroom_EnemyPink"))))