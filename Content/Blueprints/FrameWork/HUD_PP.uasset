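; HUD Blueprint that manages the game's in-game HUD, pause screen and game-over screen widgets.
; BeginPlay creates the HUD and pause widgets, while GameOver swaps the HUD for a game-over screen with UI-only input.
; Paused toggles game pause, the pause widget, cursor and input mode, centering the mouse using the screen center cached in DrawHUD.
; The remaining gameplay query functions are empty stubs returning defaults.
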(event `self.ReceiveBeginPlay`
  (bind _returnvalue (`|CreateWidget` "/Game/Blueprints/Widgets/WBP_PauseScreen.WBP_PauseScreen_C"))
  (set `self.PAUSEREF` _returnvalue)
  (bind _returnvalue_2 (`|CreateWidget` "/Game/Blueprints/Widgets/WBP_HUD.WBP_HUD_C"))
  (bind _output_get (set `self.HUDREF` _returnvalue_2))
  (`UserWidget.AddToViewport` _output_get 0)
  (`WidgetBlueprintLibrary.SetInputMode_GameOnly` (`GameplayStatics.GetPlayerController` 0)))

(event `/Game/Blueprints/FrameWork/Interface_PP.GameOver`
  (bind _returnvalue (`GameplayStatics.GetPlayerController` 0))
  (`Widget.RemoveFromParent` (`self.HUDREF`))
  (bind _returnvalue_2 (`|CreateWidget` "/Game/Blueprints/Widgets/WBP_GameOver.WBP_GameOver_C"))
  (`UserWidget.AddToViewport` _returnvalue_2 0)
  (set `PlayerController.bShowMouseCursor` true _returnvalue)
  (set `PlayerController.bEnableClickEvents` true _returnvalue)
  (`WidgetBlueprintLibrary.SetInputMode_UIOnlyEx` _returnvalue _returnvalue_2))

(event `/Game/Blueprints/FrameWork/Interface_PP.Paused`
  (bind _returnvalue (`GameplayStatics.GetPlayerController` 0))
  (bind _pauseref (`self.PAUSEREF`))
  (if (`GameplayStatics.IsGamePaused`)
    (`GameplayStatics.SetGamePaused` false)
    (`Widget.RemoveFromParent` _pauseref)
    (set `PlayerController.bShowMouseCursor` false _returnvalue)
    (set `PlayerController.bEnableClickEvents` false _returnvalue)
    (`WidgetBlueprintLibrary.SetInputMode_GameOnly` _returnvalue)
    (else
      (`GameplayStatics.SetGamePaused` true)
      (`UserWidget.AddToViewport` _pauseref 0)
      (set `PlayerController.bShowMouseCursor` true _returnvalue)
      (set `PlayerController.bEnableClickEvents` true _returnvalue)
      (`PlayerController.SetMouseLocation` _returnvalue (`self.CentreX`) (`self.CentreY`))
      (`WidgetBlueprintLibrary.SetInputMode_GameAndUIEx` _returnvalue _pauseref)
      (`/Game/Blueprints/Widgets/WBP_PauseScreen.ResetLooks` (`self.PAUSEREF`)))))

(event `self.ReceiveDrawHUD`
  (params (SizeX :type Integer) (SizeY :type Integer))
  (set `self.CentreX` (/ SizeX 2))
  (set `self.CentreY` (/ SizeY 2)))

(fn `CheckForSpaceHUD`
  (returns (`AnySpace?` :type Boolean) (EmptySlot :type "/Game/Blueprints/Widgets/WBP_HotbarSlot Object Reference"))
  (return false null))

(fn `ChooseRandomEnemy`
  (params (AlreadySelectedEnemy :type "/Game/Blueprints/Actors/Enemies/BP_Enemy Class Reference"))
  (returns (ChosenEnemy :type "/Game/Blueprints/Actors/Enemies/BP_Enemy Class Reference") (SpawnModifiers :type "/Game/Blueprints/FrameWork/S_EnemyModifiers Structure"))
  (return null))

(fn `GetChestItem`
  (params (Rarity :type Integer))
  (returns (ItemReceived :type "/Game/Blueprints/Actors/Interactables/Pickups/BP_PickUp Class Reference"))
  (return null))

(fn `GetPlayerStats`
  (returns (PlayerStats :type "/Game/Blueprints/FrameWork/S_PlayerStats Structure") (CurrentTime :type "Float (double-precision)"))
  (return (struct) 0.0))

(fn `GetRandomLevel`
  (params (LevelType :type "/Game/Blueprints/FrameWork/Enum_PortalTypes Enum" :default "NewEnumerator0"))
  (returns (ChosenLevel :type Name))
  (return "None"))

(fn `UserConstructionScript`)