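; Game instance that holds roguelike run state across levels: player stats, timer and current level.
; Its events broadcast level start, completion, game over and victory through Interface_PP; level 20 switches portals to boss, and a failsafe completes enemy-free levels.
; Helper functions pick random levels by type, chest loot by rarity and enemies with level-scaled modifiers.
; The PPSave1 save slot supplies volume settings and records beating the game.
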(event `/Game/Blueprints/FrameWork/Interface_PP.GameComplete`
  (`|ExecutionSequence`
    (:`then_0`
      (bind _outactors (`GameplayStatics.GetAllActorsWithInterface` "/Game/Blueprints/FrameWork/Interface_PP.Interface_PP_C"))
      (for _array_element _outactors
        (message `/Game/Blueprints/FrameWork/Interface_PP.GameComplete` _array_element)))
    (:`then_1`
      (bind _returnvalue (`GameplayStatics.LoadGameFromSlot` "PPSave1"))
      (bind _asbp_save_game (cast `/Game/Blueprints/FrameWork/BP_SaveGame` _returnvalue))
      (set `/Game/Blueprints/FrameWork/BP_SaveGame.HaveBeatenGame` true _asbp_save_game)
      (`GameplayStatics.SaveGameToSlot` _asbp_save_game "PPSave1"))
    (:`then_2`
      (`GameplayStatics.OpenLevelBySoftObjectPtr` "/Game/Levels/TheHubPostGame.TheHubPostGame"))))

(event `/Game/Blueprints/FrameWork/Interface_PP.SavePlayerStats`
  (params (PlayerPreviousStats :type "/Game/Blueprints/FrameWork/S_PlayerStats Structure") (CurrentTime :type "Float (double-precision)"))
  ; Save Player Data between levels
  (set `self.PlayerStats` (make `/Game/Blueprints/FrameWork/S_PlayerStats` PlayerPreviousStats_Health_2_C92201914B0B425E46F9998F44FA4AA4 PlayerPreviousStats_MaxHealth_18_E7A9C1C14A7F2833BA2D808E4C4C37F6 PlayerPreviousStats_Money_4_237A31944AACA64C550715AD4F0FA176 PlayerPreviousStats_InvSlot1_7_324CA6E94285E51DC02922BBFE43F735 PlayerPreviousStats_InvSlot2_12_B017CE3A4F1FDF0E2AD024B0E5B18C6A PlayerPreviousStats_InvSlot3_13_B89400F44A7E449D972B3CBF08934FF7 PlayerPreviousStats_InvSlot4_14_7AA60E214CF7CE25E20C5B85EE21E9F3 PlayerPreviousStats_InvSlot5_15_D9E449944204A36FA1A1539F624F9FBD PlayerPreviousStats_CurrentSlot_21_1D923B014E5F65289E17C68BA1C25990))
  (set `self.CurrentTime` CurrentTime))

(event `/Game/Blueprints/FrameWork/Interface_PP.LevelComplete`
  ; Activate portals upon level complete (check current level and set all portals to boss if high enough)
  (`GameplayStatics.PlaySound2D` "/Game/Audio/A_PortalOpen.A_PortalOpen" 1.0 1.0 0.0 null null)
  (bind _ashud_pp (cast `/Game/Blueprints/FrameWork/HUD_PP` (`PlayerController.GetHUD` (`GameplayStatics.GetPlayerController` 0))))
  (`/Game/Blueprints/Widgets/WBP_HUD.LevelComplete` (`/Game/Blueprints/FrameWork/HUD_PP.HUDREF` _ashud_pp))
  (if (== (`self.CurrentLevel`) 20)
    (`KismetSystemLibrary.PrintString` "LEVEL 20 YEAAAAAAAH")
    (bind _outactors (`GameplayStatics.GetAllActorsOfClass` "/Game/Blueprints/Actors/BP_Portal.BP_Portal_C"))
    (for _array_element _outactors
      (set `/Game/Blueprints/Actors/BP_Portal.PortalType` "NewEnumerator4" _array_element)
      (`KismetSystemLibrary.Delay` 0.2)
      (bind _outactors_2 (`GameplayStatics.GetAllActorsWithInterface` "/Game/Blueprints/FrameWork/Interface_PP.Interface_PP_C"))
      (for _array_element_2 _outactors_2
        (message `/Game/Blueprints/FrameWork/Interface_PP.LevelComplete` _array_element_2)))
    (else
      (bind _outactors_3 (`GameplayStatics.GetAllActorsWithInterface` "/Game/Blueprints/FrameWork/Interface_PP.Interface_PP_C"))
      (for _array_element_3 _outactors_3
        (message `/Game/Blueprints/FrameWork/Interface_PP.LevelComplete` _array_element_3)))))

(event `/Game/Blueprints/FrameWork/Interface_PP.GameOver`
  ; Game Over (reset variables)
  (set `self.PlayerStats` (`self.FreshStats`))
  (set `self.CurrentTime` 0.0)
  (set `self.CurrentLevel` 0)
  (bind _outactors (`GameplayStatics.GetAllActorsWithInterface` "/Game/Blueprints/FrameWork/Interface_PP.Interface_PP_C"))
  (for _array_element _outactors
    (message `/Game/Blueprints/FrameWork/Interface_PP.GameOver` _array_element)))

(event `/Game/Blueprints/FrameWork/Interface_PP.ChangedVolume`
  (params (NewVolume :type "Float (double-precision)") (`Music(True)orSFX(False)` :type Boolean))
  (bind _returnvalue (`KismetMathLibrary.FClamp` (/ NewVolume 100.0) 0.001))
  ; Volume Change
  (if `Music(True)orSFX(False)`
    (`GameplayStatics.SetSoundMixClassOverride` "/Game/Audio/PP_BaseSoundClassMix.PP_BaseSoundClassMix" "/Engine/EngineSounds/Music.Music" _returnvalue 1.0 0.0)
    (else
      (`GameplayStatics.SetSoundMixClassOverride` "/Game/Audio/PP_BaseSoundClassMix.PP_BaseSoundClassMix" "/Engine/EngineSounds/SFX.SFX" _returnvalue 1.0 0.0))))

(event `/Game/Blueprints/FrameWork/Interface_PP.LevelStart`
  ; LevelStart
  (set `self.CurrentChallengeFailed?` false)
  (bind _returnvalue (`GameplayStatics.GetCurrentLevelName` true))
  (set `self.PreviousLevelName` (`KismetStringLibrary.Conv_StringToName` _returnvalue))
  (bind _outactors (`GameplayStatics.GetAllActorsWithInterface` "/Game/Blueprints/FrameWork/Interface_PP.Interface_PP_C"))
  (for _array_element _outactors
    (message `/Game/Blueprints/FrameWork/Interface_PP.LevelStart` _array_element)))

(event `CheckForEnemies`
  ; Enemy Check Failsafe
  (`KismetSystemLibrary.Delay` 1.0)
  (bind _outactors (`GameplayStatics.GetAllActorsOfClass` "/Game/Blueprints/Actors/Enemies/BP_Enemy.BP_Enemy_C"))
  (if (== (`KismetArrayLibrary.Array_Length` _outactors) 0)
    (bind _outactors_2 (`GameplayStatics.GetAllActorsOfClass` "/Game/Blueprints/Actors/BP_Portal.BP_Portal_C"))
    (for _array_element _outactors_2
      (if (not (`/Game/Blueprints/Actors/BP_Portal.PortalActive` _array_element))
        (`self.LevelComplete`)
        (break)))))

(event `self.ReceiveInit`
  (bind _returnvalue (`GameplayStatics.DoesSaveGameExist` "PPSave1"))
  (if _returnvalue
    (bind _returnvalue_2 (`GameplayStatics.LoadGameFromSlot` "PPSave1"))
    (bind _asbp_save_game (cast `/Game/Blueprints/FrameWork/BP_SaveGame` _returnvalue_2))
    (`KismetSystemLibrary.Delay` 0.2)
    (`/Game/Blueprints/FrameWork/Interface_PP.ChangedVolume` self (`/Game/Blueprints/FrameWork/BP_SaveGame.Music_Volume` _asbp_save_game) true)
    (`/Game/Blueprints/FrameWork/Interface_PP.ChangedVolume` self (`/Game/Blueprints/FrameWork/BP_SaveGame.SFX_Volume` _asbp_save_game) false)
    (else
      (bind _returnvalue_3 (`GameplayStatics.CreateSaveGameObject` "/Game/Blueprints/FrameWork/BP_SaveGame.BP_SaveGame_C"))
      (set `/Game/Blueprints/FrameWork/BP_SaveGame.MagnumShards` 0.0 _returnvalue_3)
      (set `/Game/Blueprints/FrameWork/BP_SaveGame.SpeedrunningTimerToggle` false _returnvalue_3)
      (set `/Game/Blueprints/FrameWork/BP_SaveGame.HaveBeatenGame` false _returnvalue_3)
      (set `/Game/Blueprints/FrameWork/BP_SaveGame.HeadbobToggle` true _returnvalue_3)
      (`GameplayStatics.SaveGameToSlot` _returnvalue_3 "PPSave1")
      (`KismetSystemLibrary.PrintString` "No Save Detected, Giving Fresh Data!" true true (struct :`R` 0.703342 :`B` 1.0 :`A` 1.0) 10.0))))

(fn `CheckForSpaceHUD`
  (returns (`AnySpace?` :type Boolean) (EmptySlot :type "/Game/Blueprints/Widgets/WBP_HotbarSlot Object Reference"))
  (return false null))

(fn `ChooseRandomEnemy`
  (params (AlreadySelectedEnemy :type "/Game/Blueprints/Actors/Enemies/BP_Enemy Class Reference"))
  (returns (ChosenEnemy :type "/Game/Blueprints/Actors/Enemies/BP_Enemy Class Reference") (SpawnModifiers :type "/Game/Blueprints/FrameWork/S_EnemyModifiers Structure"))
  (bind _returnvalue (+ 1.0 (* (`self.CurrentLevel`) (`self.AttackModiefierAdd`))))
  (bind _returnvalue_2 (+ 1.0 (* (`self.CurrentLevel`) (`self.HealthModifierAdd`))))
  (if (== AlreadySelectedEnemy null)
    (return (`KismetArrayLibrary.Array_Random` (`self.EnemyPool`)) (make `/Game/Blueprints/FrameWork/S_EnemyModifiers` _returnvalue_2 _returnvalue 1.0))
    (else
      (return AlreadySelectedEnemy (make `/Game/Blueprints/FrameWork/S_EnemyModifiers` _returnvalue_2 _returnvalue 1.0)))))

(fn `GetChestItem`
  (params (Rarity :type Integer))
  (returns (ItemReceived :type "/Game/Blueprints/Actors/Interactables/Pickups/BP_PickUp Class Reference"))
  (bind _itemsofrarity (`self.ItemsOfRarity`))
  (bind _output_pickupactor (break `/Game/Blueprints/FrameWork/S_Lootpool` (`|GetArrayItem` _itemsofrarity)))
  (`KismetSystemLibrary.PrintString` (`KismetStringLibrary.Conv_IntToString` Rarity))
  (`KismetArrayLibrary.Array_Clear` (`self.ItemsOfRarity`))
  (for _array_element (`self.Lootpool Array`)
    (if (== (`.LootType_19_B1F8B1F545B008D9B83D668F31306022` (break `/Game/Blueprints/FrameWork/S_Lootpool` _array_element)) Rarity)
      (`KismetArrayLibrary.Array_Add` (`self.ItemsOfRarity`) _array_element)))
  (`KismetArrayLibrary.Array_Shuffle` _itemsofrarity)
  (return _output_pickupactor))

(fn `GetPlayerStats`
  (returns (PlayerStats :type "/Game/Blueprints/FrameWork/S_PlayerStats Structure") (CurrentTime :type "Float (double-precision)"))
  (return (`self.PlayerStats`) (`self.CurrentTime`)))

(fn `GetRandomLevel`
  (params (LevelType :type "/Game/Blueprints/FrameWork/Enum_PortalTypes Enum" :default "NewEnumerator0"))
  (returns (ChosenLevel :type Name))
  (bind _levelsoftype (`self.LevelsOfType`))
  (bind _output_levelname (break `/Game/Blueprints/FrameWork/S_LevelPool` (`|GetArrayItem` _levelsoftype)))
  (bind _output_levelname_2 (break `/Game/Blueprints/FrameWork/S_LevelPool` (`|GetArrayItem` _levelsoftype 1)))
  (`KismetArrayLibrary.Array_Clear` (`self.LevelsOfType`))
  (for _array_element (`self.LevelArray`)
    (if (== (`.Type_8_B20CC43447C56D43A33B53BF95E2FAC8` (break `/Game/Blueprints/FrameWork/S_LevelPool` _array_element)) (`KismetMathLibrary.Conv_ByteToInt` LevelType))
      (`KismetArrayLibrary.Array_Add` (`self.LevelsOfType`) _array_element)))
  (`KismetArrayLibrary.Array_Shuffle` _levelsoftype)
  (if (== (`self.PreviousLevelName`) _output_levelname)
    (return _output_levelname_2)
    (else
      (return _output_levelname))))